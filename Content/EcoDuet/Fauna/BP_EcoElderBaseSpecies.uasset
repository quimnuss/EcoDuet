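; Base elder character for an EcoDuet fauna species, owning its population of child animals and its generalized Lotka-Volterra (GLV) parameters.
; It spawns or damages children to match a given density, adjusts game-mode density when children are added or player-killed, and handles extinction.
; Selectable mini cubes represent growth rate and up to four species relations; resizing one edits that parameter and recolors it.
; TickGLV delegates the simulation step to EcoGLVActor.
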(event `self.ReceiveBeginPlay`
  (`parent.ReceiveBeginPlay`)
  (bind _returnvalue (`GameplayStatics.GetActorOfClass` "/Game/EcoDuet/Fauna/BP_EcoSpeciesManager.BP_EcoSpeciesManager_C"))
  (set `self.EcoSpeciesManager` _returnvalue)
  (bind _outactors (`GameplayStatics.GetAllActorsOfClass` (`self.Children Class`)))
  (set `self.EcoChildren` _outactors)
  (`KismetSystemLibrary.DelayUntilNextTick`)
  (`self.BuildInteractionCubes`))

(event `AddChildrenPlayer`
  (params (NewChild :type "Actor Object Reference"))
  (`KismetArrayLibrary.Array_Add` (`self.EcoChildren`) NewChild))

(event `IncreaseCube`
  (bind _output (`|GetArrayItem` (`self.InteractionCubes`) (`self.TargetCubeIndex`)))
  (bind _ecominicube (`/Game/EcoDuet/Actors/BP_EcoInteractionCube.EcoMiniCube` _output))
  ;[1 1 1] GLV Interaction
  (`SceneComponent.SetWorldScale3D` _ecominicube (+ (`SceneComponent.K2_GetComponentScale` _ecominicube) 0.05))
  (bind _newglvparametervalue (`self.UpdateGLVParameters` _output 0.1))
  (`/Game/EcoDuet/Actors/BP_EcoInteractionCube.ColorLights` _output _newglvparametervalue))

(event `DecreaseCube`
  (bind _output (`|GetArrayItem` (`self.InteractionCubes`) (`self.TargetCubeIndex`)))
  (bind _ecominicube (`/Game/EcoDuet/Actors/BP_EcoInteractionCube.EcoMiniCube` _output))
  ;[1 1 1] GLV Interaction
  (`SceneComponent.SetWorldScale3D` _ecominicube (- (`SceneComponent.K2_GetComponentScale` _ecominicube) 0.05))
  (bind _newglvparametervalue (`self.UpdateGLVParameters` _output -0.1))
  (`/Game/EcoDuet/Actors/BP_EcoInteractionCube.ColorLights` _output _newglvparametervalue))

(event `ChangeTargetCube`
  (params (Forward :type Boolean))
  (bind _targetcubeindex (`self.TargetCubeIndex`))
  (bind _interactioncubes (`self.InteractionCubes`))
  (bind _returnvalue (`KismetArrayLibrary.Array_Length` _interactioncubes))
  ;[1 1 1] GLV Interaction
  (`/Game/EcoDuet/Actors/BP_EcoInteractionCube.Deselect` (`|GetArrayItem` _interactioncubes _targetcubeindex))
  (if Forward
    (set `self.TargetCubeIndex` (mod (+ _targetcubeindex 1) _returnvalue))
    (else
      (set `self.TargetCubeIndex` (mod (+ (- _targetcubeindex 1) _returnvalue) _returnvalue))))
  (`/Game/EcoDuet/Actors/BP_EcoInteractionCube.Select` (`|GetArrayItem` (`self.InteractionCubes`) (`self.TargetCubeIndex`))))

(event `ShowAnimalIcons`
  ;[1 1 1] GLV Interaction
  (for _array_element (`self.InteractionCubes`)
    (`SceneComponent.SetVisibility` (`/Game/EcoDuet/Actors/BP_EcoInteractionCube.DefaultSceneRoot` _array_element) true false)
    (`SceneComponent.SetVisibility` (`/Game/EcoDuet/Actors/BP_EcoInteractionCube.EcoMiniCube` _array_element) true false)))

(event `HideAnimalIcons`
  ;[1 1 1] GLV Interaction
  (for _array_element (`self.InteractionCubes`)
    (`SceneComponent.SetVisibility` (`/Game/EcoDuet/Actors/BP_EcoInteractionCube.DefaultSceneRoot` _array_element) false false)
    (`SceneComponent.SetVisibility` (`/Game/EcoDuet/Actors/BP_EcoInteractionCube.EcoMiniCube` _array_element) false false)))

(fn `AddEcoFaunaChild`
  (params (NewChild :type "Actor Object Reference"))
  (bind _isvalidecochild (`self.IsValidEcoChild` NewChild))
  (if _isvalidecochild
    (`KismetArrayLibrary.Array_Add` (`self.EcoChildren`) NewChild)
    (`self.AddSpeciesDensity` (`self.EcoName`) 1.0)))

(fn `AddMiniCube`
  (params (InteractionCube :type "ChildActorComponent Object Reference") (Material :type "MaterialInterface Object Reference") (EcoElderName :type Name) (isR :type Boolean) (InitialValue :type "Float (double-precision)"))
  (bind _asbp_eco_interaction_cube (cast `/Game/EcoDuet/Actors/BP_EcoInteractionCube` (`ChildActorComponent.ChildActor` InteractionCube) :!pure true))
  (set `/Game/EcoDuet/Actors/BP_EcoInteractionCube.IsRCube` isR _asbp_eco_interaction_cube)
  (set `/Game/EcoDuet/Actors/BP_EcoInteractionCube.EcoElderName` EcoElderName _asbp_eco_interaction_cube)
  (`/Game/EcoDuet/Actors/BP_EcoInteractionCube.ColorLights` _asbp_eco_interaction_cube InitialValue)
  (`/Engine/EditorBlueprintResources/StandardMacros.IsValid` _asbp_eco_interaction_cube
    (:`Is Valid`
      (`PrimitiveComponent.SetMaterial` (`/Game/EcoDuet/Actors/BP_EcoInteractionCube.EcoMiniCube` _asbp_eco_interaction_cube) 0 Material)
      (`KismetArrayLibrary.Array_Add` (`self.InteractionCubes`) _asbp_eco_interaction_cube))))

(fn `AddSpeciesDensity`
  (params (SpeciesName :type "Name (by ref)") (DeltaDensity :type "Float (double-precision)"))
  (bind _ecologydensitiesmap (`/Game/EcoDuet/GameLogic/BP_EcoGameModeHome.EcologyDensitiesMap` (cast `/Game/EcoDuet/GameLogic/BP_EcoGameModeHome` (`GameplayStatics.GetGameMode`) :!pure true)))
  (`BlueprintMapLibrary.Map_Add` _ecologydensitiesmap SpeciesName (+ DeltaDensity (`BlueprintMapLibrary.Map_Find` _ecologydensitiesmap SpeciesName))))

(fn `BuildInteractionCubes`
  (locals (CubeIndex :type Integer))
  (bind _ecoelderrelationvector (`EcoGLVActorComponent.EcoElderRelationVector` (`self.EcoGLVActor`)))
  (`self.AddMiniCube` (`self.InteractionCubeR`) (`self.CubeMaterial`) "R" true (`EcoGLVActorComponent.rate` (`self.EcoGLVActor`)))
  (`/Game/EcoDuet/Actors/BP_EcoInteractionCube.Select` (`|GetArrayItem` (`self.InteractionCubes`) (`self.TargetCubeIndex`)))
  (bind _keys (`BlueprintMapLibrary.Map_Keys` _ecoelderrelationvector))
  (for _array_element _keys
    (bind (_value _returnvalue) (`BlueprintMapLibrary.Map_Find` _ecoelderrelationvector _array_element))
    (bind (_value_2 _returnvalue_2) (`BlueprintMapLibrary.Map_Find` (`/Game/EcoDuet/Fauna/BP_EcoSpeciesManager.ElderMap` (`self.EcoSpeciesManager`)) _array_element))
    (if (and (>= (`KismetMathLibrary.Abs` _value) 0.001) _returnvalue _returnvalue_2)
      (`|ExecutionSequence`
        (:`then_0`
          ;[1 1 1] TODO add to interaction cubes around here and loop array
          (switch `int` (`local.CubeIndex`)
            (:`0`
              (bind _cubematerial (`/Game/EcoDuet/Fauna/BP_EcoElderBaseSpecies.CubeMaterial` _value_2))
              (`self.AddMiniCube` (`self.InteractionCube0`) _cubematerial _array_element false _value))
            (:`1`
              (`self.AddMiniCube` (`self.InteractionCube1`) _cubematerial _array_element false _value))
            (:`2`
              (`self.AddMiniCube` (`self.InteractionCube2`) _cubematerial _array_element false _value))
            (:`3`
              (`self.AddMiniCube` (`self.InteractionCube3`) _cubematerial _array_element false _value))))
        (:`then_1`
          (`/Engine/EditorBlueprintResources/StandardMacros.IncrementInt` (`local.CubeIndex`)))))))

(fn `DamageArrayActors`
  (params (TargetLength :type Integer) (Array :type "Array of Actor Object Reference"))
  (bind _returnvalue (`KismetArrayLibrary.Array_LastIndex` Array))
  (while (> (`KismetArrayLibrary.Array_Length` Array) TargetLength)
    (`GameplayStatics.ApplyDamage` (`|GetArrayItem` Array _returnvalue) 100.0 null self)
    (`KismetArrayLibrary.Array_Remove` Array _returnvalue)))

(fn `DestroyArrayItems`
  (params (TargetLength :type Integer) (Array :type "Array of Actor Object Reference"))
  (bind _returnvalue (`KismetArrayLibrary.Array_LastIndex` Array))
  (while (> (`KismetArrayLibrary.Array_Length` Array) TargetLength)
    (`self.K2_DestroyActor` (`|GetArrayItem` Array _returnvalue))
    (`KismetArrayLibrary.Array_Remove` Array _returnvalue)))

(fn `Die`
  (`CharacterMovementComponent.DisableMovement` (`self.CharacterMovement`))
  (`GameplayStatics.PlaySoundAtLocation` (`self.Death Sound`) (`self.K2_GetActorLocation`) (struct) 1.0 1.0 0.0 "/Game/EcoDuet/Media/EcoFaunaSoundAttenuation.EcoFaunaSoundAttenuation" null null null)
  (`SkeletalMeshComponent.PlayAnimation` (`self.Mesh`) (`self.DeathSequence`) false)
  (`self.SetLifeSpan` 5.0))

(fn `IsValidEcoChild`
  (params (EcoChild :type "Actor Object Reference"))
  (returns (IsValidEcoChild :type Boolean))
  (bind _returnvalue (`GameplayStatics.GetObjectClass` EcoChild))
  (bind _children_class (`self.Children Class`))
  (bind _returnvalue_2 (== _returnvalue _children_class))
  (if (not _returnvalue_2)
    (`KismetSystemLibrary.PrintText` (`|FormatText` "New actor {new actor class} is not of class {child class}" (`KismetSystemLibrary.GetClassDisplayName` _children_class) (`KismetSystemLibrary.GetClassDisplayName` _returnvalue))))
  (return _returnvalue_2))

(fn `KillChildByPlayer`
  (params (EcoFaunaChildToKill :type "/Game/EcoDuet/Fauna/BP_EcoFaunaBaseCharacter Object Reference") (Instigator :type "Actor Object Reference"))
  (bind _returnvalue (`KismetArrayLibrary.Array_RemoveItem` (`self.EcoChildren`) EcoFaunaChildToKill))
  (if _returnvalue
    (`self.AddSpeciesDensity` (`self.EcoName`) -1.0)
    (`GameplayStatics.ApplyDamage` EcoFaunaChildToKill 100.0 null Instigator)))

(fn `KillChildren`
  (params (NumChildren :type Integer))
  (locals (TargetLenght :type Integer))
  (bind _ecochildren (`self.EcoChildren`))
  (bind _output_get (set `local.TargetLenght` (- (`KismetArrayLibrary.Array_Length` _ecochildren) NumChildren)))
  (`self.DamageArrayActors` _output_get _ecochildren))

(fn `MakeSpeciesExtinct`
  (`self.KillChildren` (`KismetArrayLibrary.Array_Length` (`self.EcoChildren`)))
  (set `self.IsDeadSpecies` true)
  (`self.Die`))

(fn `SpawnChildren`
  (params (NumChildren :type Integer))
  (`/Engine/EditorBlueprintResources/StandardMacros.Do N` NumChildren
    (:`Exit`
      (bind _returnvalue (`|SpawnActorFromClass` (`self.Children Class`) (`self.GetTransform` self) "AdjustIfPossibleButAlwaysSpawn" "SelectDefaultAtRuntime" null self))
      (`KismetArrayLibrary.Array_Add` (`self.EcoChildren`) _returnvalue))))

(fn `SpawnChildrenLogic`
  (params (NewDensity :type "Float (double-precision)"))
  (bind _returnvalue (- (`KismetMathLibrary.FCeil` NewDensity) (`KismetArrayLibrary.Array_Length` (`self.EcoChildren`))))
  (if (`self.IsDeadSpecies`)
    _
    (elif (== _returnvalue 0)
      _
      (elif (> _returnvalue 0)
        (`self.SpawnChildren` (`KismetMathLibrary.Clamp` _returnvalue 0 10))
        (else
          (bind _result (`/Engine/EditorBlueprintResources/StandardMacros.NegateInt` _returnvalue)
            (:`  `
              (`self.KillChildren` _result))))))))

(fn `TickGLV`
  (params (Densities :type "Map of Name to Float (double-precision)") (`Delta Time` :type "Float (double-precision)"))
  (returns (NewDensity :type "Float (double-precision)"))
  (bind _returnvalue (`EcoGLVActorComponent.VoltkaTick` (`self.EcoGLVActor`) `Delta Time` Densities))
  (return _returnvalue))

(fn `UpdateGLVParameters`
  (params (InteractionCube :type "/Game/EcoDuet/Actors/BP_EcoInteractionCube Object Reference") (Delta :type "Float (double-precision)"))
  (returns (NewGLVParameterValue :type "Float (double-precision)"))
  (bind _ecoglvactor (`self.EcoGLVActor`))
  (bind _ecoeldername (`/Game/EcoDuet/Actors/BP_EcoInteractionCube.EcoElderName` InteractionCube))
  (bind _ecoelderrelationvector (`EcoGLVActorComponent.EcoElderRelationVector` _ecoglvactor))
  (bind _returnvalue (+ Delta (`BlueprintMapLibrary.Map_Find` _ecoelderrelationvector _ecoeldername)))
  (if (`/Game/EcoDuet/Actors/BP_EcoInteractionCube.IsRCube` InteractionCube)
    (bind _output_get (set `EcoGLVActorComponent.rate` (+ Delta (`EcoGLVActorComponent.rate` _ecoglvactor)) _ecoglvactor))
    (return _output_get)
    (else
      (`BlueprintMapLibrary.Map_Add` _ecoelderrelationvector _ecoeldername _returnvalue)
      (return _returnvalue))))

(fn `UserConstructionScript`
  (`parent.UserConstructionScript`))