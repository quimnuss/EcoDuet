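; Ecology manager that tracks every species' elder actor and drives population simulation, spawning and extinction.
; A looping timer ticks each living elder's GLV (Lotka-Volterra) actor and writes the new densities to BP_EcoGameModeHome's map.
; A second, slightly slower timer reads that map to spawn children per elder or signal extinction below a threshold, removing that elder from the living list.
; AddElder registers new elders and refreshes all elders' cubes.
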(event `self.ReceiveBeginPlay`
  (add `self.SpeciesExtinct` (delegate `RemoveAliveElder`))
  (bind _returnvalue (`KismetSystemLibrary.K2_SetTimerDelegate` (delegate `GLVTick`) 1.0 true))
  (set `self.GLVTickTimer` _returnvalue)
  (bind _returnvalue_2 (`KismetSystemLibrary.K2_SetTimer` null "SpawnSpeciesLogic" 1.2 true))
  (set `self.SyncSpeciesToDensitiesTimer` _returnvalue_2)
  (bind _outactors (`GameplayStatics.GetAllActorsOfClass` "/Game/EcoDuet/Fauna/BP_EcoElderBaseSpecies.BP_EcoElderBaseSpecies_C"))
  (bind _output_get (set `self.AllEcoElders` _outactors))
  (bind _output_get_2 (set `self.EcoEldersAlive` _output_get))
  (for _array_element _output_get_2
    (`BlueprintMapLibrary.Map_Add` (`self.ElderMap`) (`/Game/EcoDuet/Fauna/BP_EcoElderBaseSpecies.EcoSpecies` _array_element) _array_element)))

(event `RemoveAliveElder` :!signature `self.SpeciesExtinct`
  (params (Species :type "EEcoSpeciesType Enum" :default "EcoNone"))
  (`self.ExtinctElder` Species))

(event `GLVTick`
  (bind _asbp_eco_game_mode_home (cast `/Game/EcoDuet/GameLogic/BP_EcoGameModeHome` (`GameplayStatics.GetGameMode`) :!pure true))
  (bind _newspeciesdensities (`self.GLVTickFunction` 1.0 (`/Game/EcoDuet/GameLogic/BP_EcoGameModeHome.EcologySpeciesDensitiesMap` _asbp_eco_game_mode_home)))
  (set `/Game/EcoDuet/GameLogic/BP_EcoGameModeHome.EcologySpeciesDensitiesMap` _newspeciesdensities _asbp_eco_game_mode_home))

(fn `AddElder`
  (params (NewElder :type "/Game/EcoDuet/Fauna/BP_EcoElderBaseSpecies Object Reference"))
  (bind _eldermap (`self.ElderMap`))
  (bind _ecospecies (`/Game/EcoDuet/Fauna/BP_EcoElderBaseSpecies.EcoSpecies` NewElder))
  (`|ExecutionSequence`
    (:`then_0`
      (`KismetArrayLibrary.Array_Add` (`self.AllEcoElders`) NewElder)
      (`KismetArrayLibrary.Array_Add` (`self.EcoEldersAlive`) NewElder)
      (if (`.ReturnValue` (`BlueprintMapLibrary.Map_Find` _eldermap _ecospecies))
        (`KismetSystemLibrary.PrintText` (`|FormatText` "[EcoSpeciesManager {elder} already mapped" (`KismetStringLibrary.Conv_StringToName` (`|GetEnumeratorNameAsString` _ecospecies))))
        (else
          (`BlueprintMapLibrary.Map_Add` _eldermap _ecospecies NewElder))))
    (:`then_1`
      (`self.UpdateEldersCubes`))))

(fn `ExtinctElder`
  (params (Species :type "EEcoSpeciesType Enum" :default "EcoNone"))
  (locals (SpeciesToExtinct :type "/Game/EcoDuet/Fauna/BP_EcoElderBaseSpecies Object Reference"))
  (bind _speciestoextinct (`local.SpeciesToExtinct`))
  (bind _ecoeldersalive (`self.EcoEldersAlive`))
  (for _array_element _ecoeldersalive
    (if (`|EnumEquality` Species (`/Game/EcoDuet/Fauna/BP_EcoElderBaseSpecies.EcoSpecies` _array_element))
      (set `local.SpeciesToExtinct` _array_element)
      (break)))
  (`/Engine/EditorBlueprintResources/StandardMacros.IsValid` _speciestoextinct
    (:`Is Valid`
      (`KismetArrayLibrary.Array_RemoveItem` _ecoeldersalive _speciestoextinct)
      (`/Game/EcoDuet/Fauna/BP_EcoElderBaseSpecies.MakeSpeciesExtinct` _speciestoextinct))))

(fn `GLVTickFunction`
  (params (DeltaTime :type "Float (double-precision)") (SpeciesDensities :type "Map of EEcoSpeciesType Enum to Float (double-precision)"))
  (returns (NewSpeciesDensities :type "Map of EEcoSpeciesType Enum to Float (double-precision)"))
  (locals (NextDensities :type "Map of Name to Float (double-precision)") (NextSpeciesDensities :type "Map of EEcoSpeciesType Enum to Float (double-precision)"))
  (for _array_element (`self.EcoEldersAlive`)
    (bind _returnvalue (`EcoGLVActorComponent.VoltkaSpeciesTick` (`/Game/EcoDuet/Fauna/BP_EcoElderBaseSpecies.EcoGLVActor` _array_element) 0.0 SpeciesDensities))
    (`BlueprintMapLibrary.Map_Add` (`local.NextSpeciesDensities`) (`/Game/EcoDuet/Fauna/BP_EcoElderBaseSpecies.EcoSpecies` _array_element) _returnvalue))
  (return (`local.NextSpeciesDensities`)))

(fn `SpawnSpeciesLogic`
  (for _array_element (`self.EcoEldersAlive`)
    (bind _ecospecies (`/Game/EcoDuet/Fauna/BP_EcoElderBaseSpecies.EcoSpecies` _array_element))
    (bind (_value _returnvalue) (`BlueprintMapLibrary.Map_Find` (`/Game/EcoDuet/GameLogic/BP_EcoGameModeHome.EcologySpeciesDensitiesMap` (cast `/Game/EcoDuet/GameLogic/BP_EcoGameModeHome` (`GameplayStatics.GetGameMode`) :!pure true)) _ecospecies))
    (if _returnvalue
      (if (< _value 0.1)
        (`self.SpeciesExtinct` (`/Game/EcoDuet/Fauna/BP_EcoElderBaseSpecies.EcoSpecies` _array_element))
        (else
          (`/Game/EcoDuet/Fauna/BP_EcoElderBaseSpecies.SpawnChildrenLogic` _array_element _value)))
      (else
        (`KismetSystemLibrary.PrintString` (`KismetTextLibrary.Conv_TextToString` (`|FormatText` "SpawnSpeciesLogic: Unknown Elder Class {elder}" (`|GetEnumeratorNameAsString` _ecospecies))))))))

(fn `UpdateEldersCubes`
  (for _array_element (`self.AllEcoElders`)
    (`/Game/EcoDuet/Fauna/BP_EcoElderBaseSpecies.UpdateElderCubes` _array_element)))

(fn `UserConstructionScript`)