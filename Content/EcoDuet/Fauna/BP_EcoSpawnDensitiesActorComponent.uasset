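; Actor component that drives fox, pig and grass spawning from the ecology densities held by the home game mode.
; On BeginPlay it caches all elder species actors and their classes, then starts a looping timer.
; Each tick of that timer switches on each elder's class display name and passes the matching EcologyDensities component (X, Y, Z) to its SpawnChildrenLogic, printing a message for unknown classes.
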(event `self.ReceiveBeginPlay`
  (bind _returnvalue (`KismetSystemLibrary.K2_SetTimer` null "SpawnSpeciesLogic" 5.0 true))
  (set `self.UpdateDensitiesTimer` _returnvalue)
  (bind _outactors (`GameplayStatics.GetAllActorsOfClass` "/Game/EcoDuet/Fauna/BP_EcoElderSpecies.BP_EcoElderSpecies_C"))
  (bind _output_get (set `self.EcoElders` _outactors))
  (for _array_element _output_get
    (`BlueprintSetLibrary.Set_Add` (`self.EldersSubClasses`) (`GameplayStatics.GetObjectClass` _array_element))))

(fn `SpawnSpeciesLogic`
  (bind (_ecologydensities_x _ecologydensities_y _ecologydensities_z) (`KismetMathLibrary.BreakVector4` (`EcoGameModeHome.EcologyDensities` (cast `EcoGameModeHome` (`GameplayStatics.GetGameMode`) :!pure true))))
  (for _array_element (`self.EcoElders`)
    (bind _returnvalue (`KismetSystemLibrary.GetClassDisplayName` (`GameplayStatics.GetObjectClass` _array_element)))
    (switch `string` _returnvalue
      (:`Default`
        (`KismetSystemLibrary.PrintString` (`KismetTextLibrary.Conv_TextToString` (`|FormatText` "Unkown Elder Class {elder}" _returnvalue))))
      (:`BP_EcoFoxElderSpecies_Child_C`
        (`/Game/EcoDuet/Fauna/BP_EcoElderSpecies.SpawnChildrenLogic` _array_element _ecologydensities_x))
      (:`BP_EcoPigElderSpecies_Child_C`
        (`/Game/EcoDuet/Fauna/BP_EcoElderSpecies.SpawnChildrenLogic` _array_element _ecologydensities_y))
      (:`BP_EcoGrassElderSpecies_Child_C`
        (`/Game/EcoDuet/Fauna/BP_EcoElderSpecies.SpawnChildrenLogic` _array_element _ecologydensities_z)))))