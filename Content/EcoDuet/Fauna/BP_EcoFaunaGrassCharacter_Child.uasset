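; Grass fauna character child Blueprint for EcoDuet that handles animated, audible spawning and death.
; On BeginPlay it runs the parent logic, then Grow plays a bush rustle sound while a timeline drives the actor's scale.
; Any damage triggers Die, which disables movement, plays a falling-tree sound and runs a shrink timeline before setting a short lifespan to remove the actor.
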(event `self.ReceiveBeginPlay`
  (`parent.ReceiveBeginPlay`)
  (`self.Grow`))

(event `Grow`
  (`GameplayStatics.PlaySoundAtLocation` "/Game/EcoDuet/Media/Fauna/bushmovement-tree.bushmovement-tree" (`self.K2_GetActorLocation`) (struct) 0.4 1.0 0.0 "/Game/EcoDuet/Media/EcoFaunaSoundAttenuation.EcoFaunaSoundAttenuation" null self null)
  (bind (_direction _growtrack) (`Timeline|GrowTimeline`)
    (:`Update`
      (`self.SetActorScale3D` _growtrack))))

(event `Die`
  (`CharacterMovementComponent.DisableMovement` (`self.CharacterMovement`))
  (`GameplayStatics.PlaySoundAtLocation` "/Game/EcoDuet/Media/Fauna/tree-falling.tree-falling" (`self.K2_GetActorLocation`) (struct) 0.4 1.0 0.0 "/Game/EcoDuet/Media/EcoFaunaSoundAttenuation.EcoFaunaSoundAttenuation" null self null)
  (bind (_direction _shrinktrack) (`Timeline|ShrinkTimeline` :!via `PlayFromStart`)
    (:`Update`
      (`self.SetActorScale3D` _shrinktrack))
    (:`Finished`
      (`self.SetLifeSpan` 1.0))))

(event `self.ReceiveAnyDamage`
  (params (Damage :type "Float (single-precision)") (DamageType :type "DamageType Object Reference") (InstigatedBy :type "Controller Object Reference") (DamageCauser :type "Actor Object Reference"))
  (`self.Die`))

(fn `UserConstructionScript`
  (`parent.UserConstructionScript`))