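; Fox fauna character child Blueprint for EcoDuet that handles the fox's death.
; Any damage triggers Die directly, as the cast of the damage causer to the elder species is left unconnected.
; Die disables movement, plays an attenuated fox sound and a one-shot death animation, then sets a short lifespan so the actor removes itself.
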(event `Die`
  (`CharacterMovementComponent.DisableMovement` (`self.CharacterMovement`))
  (`GameplayStatics.PlaySoundAtLocation` "/Game/EcoDuet/Media/Fauna/fox-hungry.fox-hungry" (`self.K2_GetActorLocation`) (struct) 0.4 1.0 0.0 "/Game/EcoDuet/Media/EcoFaunaSoundAttenuation.EcoFaunaSoundAttenuation" null null null)
  (`SkeletalMeshComponent.PlayAnimation` (`self.Mesh`) "/Game/AnimalVarietyPack/Fox/Animations/ANIM_Fox_Death.ANIM_Fox_Death" false)
  (`self.SetLifeSpan` 5.0))

(event `self.ReceiveAnyDamage`
  (params (Damage :type "Float (single-precision)") (DamageType :type "DamageType Object Reference") (InstigatedBy :type "Controller Object Reference") (DamageCauser :type "Actor Object Reference"))
  (`self.Die`))

(fn `UserConstructionScript`
  (`parent.UserConstructionScript`))