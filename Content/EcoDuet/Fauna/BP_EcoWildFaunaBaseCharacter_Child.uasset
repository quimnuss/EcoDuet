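; Wild fauna character variant that the player catches by touch, reporting to the Tennis Dungeon game mode as a caught deer.
; When BP_EcoCharacter overlaps its sphere, it calls DeerCaught, runs WireframeMe and disables the sphere's collision.
; WireframeMe freezes animation and movement, swaps every mesh material to wireframe, and spawns steam and a camera-shutter sound.
; The frozen animal stays in the world, as the destroy logic is unconnected.
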(event `self.SphereCollision.OnComponentBeginOverlap`
  (params (OverlappedComponent :type "PrimitiveComponent Object Reference") (OtherActor :type "Actor Object Reference") (OtherComp :type "PrimitiveComponent Object Reference") (OtherBodyIndex :type Integer) (bFromSweep :type Boolean) (SweepResult :type "HitResult Structure (by ref)"))
  (cast `/Game/EcoDuet/Player/BP_EcoCharacter` OtherActor)
  (`/Game/EcoDuet/GameLogic/BP_EcoGameModeTennisDungeon.DeerCaught` (cast `/Game/EcoDuet/GameLogic/BP_EcoGameModeTennisDungeon` (`GameplayStatics.GetGameMode`) :!pure true))
  (`self.WireframeMe`)
  (`PrimitiveComponent.SetCollisionEnabled` (`self.SphereCollision`) "NoCollision"))

(event `WireframeMe`
  (bind _returnvalue (`self.K2_GetActorLocation`))
  (bind _mesh (`self.Mesh`))
  (set `SkeletalMeshComponent.bPauseAnims` true (`self.Mesh`))
  (`CharacterMovementComponent.SetMovementMode` (`self.CharacterMovement`) "MOVE_None" 0)
  (for (_ _array_index) (`MeshComponent.GetMaterials` _mesh)
    (`PrimitiveComponent.SetMaterial` _mesh _array_index "/Engine/EngineDebugMaterials/WireframeMaterial.WireframeMaterial"))
  (`GameplayStatics.SpawnEmitterAtLocation` "/Game/StarterContent/Particles/P_Steam_Lit.P_Steam_Lit" _returnvalue)
  (`GameplayStatics.SpawnSoundAtLocation` "/Engine/VREditor/Sounds/UI/Camera_Shutter.Camera_Shutter" _returnvalue (struct) 1.0 1.0 0.0 null null))

(fn `UserConstructionScript`
  (`parent.UserConstructionScript`))