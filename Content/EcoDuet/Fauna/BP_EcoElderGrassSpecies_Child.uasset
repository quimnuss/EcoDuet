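; Child Blueprint of an elder grass species in EcoDuet that defines how the species spawns its offspring.
; SpawnChildren places ChildrenClass actors at random navigable points around itself, scaled down, with itself as Instigator, and records them in EcoChildren.
; Spawning adjusts for collisions but always succeeds; the event graph holds only disabled stubs, and construction defers to the parent.
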(fn `SpawnChildren`
  (params (NumChildren :type Integer))
  (for _ (range (+ NumChildren 1))
    (bind _randomlocation (`NavigationSystemV1.K2_GetRandomLocationInNavigableRadius` (`self.K2_GetActorLocation`) 1000.0 null null))
    (bind _returnvalue (`|SpawnActorFromClass` (`self.Children Class`) (`KismetMathLibrary.MakeTransform` _randomlocation (struct) (0.2 0.2 0.2)) "AdjustIfPossibleButAlwaysSpawn" "SelectDefaultAtRuntime" null self))
    (`KismetArrayLibrary.Array_Add` (`self.EcoChildren`) _returnvalue)))

(fn `UserConstructionScript`
  (`parent.UserConstructionScript`))