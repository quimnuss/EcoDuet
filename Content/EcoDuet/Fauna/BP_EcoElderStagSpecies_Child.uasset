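; Elder stag fauna species Blueprint for the EcoDuet ecology, inheriting its core behavior from a parent class.
; On BeginPlay it runs the parent logic, then assigns the deer stag death animation and sound.
; Its AddEcoFaunaChild function stores validated children in EcoChildren and increments the W channel of EcoGameModeHome's EcologyDensities vector, which acts as a population counter.
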(event `self.ReceiveBeginPlay`
  (`parent.ReceiveBeginPlay`)
  (set `self.DeathSequence` "/Game/AnimalVarietyPack/DeerStagAndDoe/Animations/ANIM_DeerStag_Death.ANIM_DeerStag_Death")
  (set `self.Death Sound` "/Game/EcoDuet/Media/Fauna/stag-death.stag-death"))

(fn `AddEcoFaunaChild`
  (params (NewChild :type "Actor Object Reference"))
  (bind _aseco_game_mode_home (cast `EcoGameModeHome` (`GameplayStatics.GetGameMode`) :!pure true))
  (bind (_ecologydensities_x _ecologydensities_y _ecologydensities_z _ecologydensities_w) (`KismetMathLibrary.BreakVector4` (`EcoGameModeHome.EcologyDensities` _aseco_game_mode_home)))
  (bind _isvalidecochild (`self.IsValidEcoChild` NewChild))
  (if _isvalidecochild
    (`KismetArrayLibrary.Array_Add` (`self.EcoChildren`) NewChild)
    (set `EcoGameModeHome.EcologyDensities` (`KismetMathLibrary.MakeVector4` _ecologydensities_x _ecologydensities_y _ecologydensities_z (+ _ecologydensities_w 1.0)) _aseco_game_mode_home)))

(fn `UserConstructionScript`
  (`parent.UserConstructionScript`))