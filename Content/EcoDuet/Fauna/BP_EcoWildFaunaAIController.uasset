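; AI controller for EcoDuet wild fauna that makes the possessed pawn wander continuously.
; On possession it moves the pawn to a random reachable point within a radius of its current location, then repeats after a short random delay, whether the move succeeds or fails.
; BeginPlay also caches all EcoCharacter actors as Players after a delay, though the roaming logic does not use them.
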(event `self.ReceiveBeginPlay`
  ;[1 1 1] switch to callbacks
  (`KismetSystemLibrary.Delay` 1.0)
  (bind _outactors (`GameplayStatics.GetAllActorsOfClass` "/Game/EcoDuet/Player/BP_EcoCharacter.BP_EcoCharacter_C"))
  (set `self.Players` _outactors))

(event `self.ReceivePossess`
  (params (PossessedPawn :type "Pawn Object Reference"))
  (`self.RoamAround`))

(event `RoamAround`
  (bind _returnvalue (`self.K2_GetPawn`))
  (`|AIMoveTo` _returnvalue (`NavigationSystemV1.K2_GetRandomReachablePointInRadius` (`self.K2_GetActorLocation` _returnvalue) (`self.Radius`) null null) null 120.0
    (:`OnSuccess`
      _)
    (:`OnFail`
      _))
  (`KismetSystemLibrary.Delay` (`KismetMathLibrary.RandomFloatInRange` 0.2 0.4))
  (`self.RoamAround`))

(fn `UserConstructionScript`)