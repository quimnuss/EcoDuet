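; BP_Follower is an EcoDuet fauna character that can follow the player and dies on its own 20 to 60 seconds after spawning.
; FollowPlayer, which BeginPlay does not start, repeats AI move requests with random acceptance radii and pauses until death.
; Kill stops movement, plays a random death animation, then disables collision and sinks the body on a timeline before destroying it.
; Getters expose its dead and sad states.
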(event `self.ReceiveBeginPlay`
  (set `self.PlayerCharacter` (`GameplayStatics.GetPlayerCharacter` 0))
  (`KismetSystemLibrary.K2_SetTimerDelegate` (delegate `Kill`) (`KismetMathLibrary.RandomFloatInRange` 20.0 60.0)))

(event `Kill`
  (bind _mesh (`self.Mesh`))
  (set `self.IsDead` true)
  (`NavMovementComponent.StopActiveMovement` (`self.CharacterMovement`))
  (switch `int` (`KismetMathLibrary.RandomInteger` 5)
    (:`Default`
      (`SkeletalMeshComponent.PlayAnimation` _mesh "/Game/AnimStarterPack/Death_Ironsights_2.Death_Ironsights_2" false :!label _label))
    (:`0`
      (goto _label))
    (:`1`
      (`SkeletalMeshComponent.PlayAnimation` _mesh "/Game/AnimStarterPack/Death_Ironsights_1.Death_Ironsights_1" false))
    (:`2`
      (`SkeletalMeshComponent.PlayAnimation` _mesh "/Game/AnimStarterPack/Death_1.Death_1" false))
    (:`3`
      (`SkeletalMeshComponent.PlayAnimation` _mesh "/Game/AnimStarterPack/Death_2.Death_2" false))
    (:`4`
      (`SkeletalMeshComponent.PlayAnimation` _mesh "/Game/AnimStarterPack/Death_2.Death_2" false)))
  (`self.submerge`))

(event `Follow Player`
  (if (not (`self.IsDead`))
    (`|AIMoveTo` self (0.0 0.0 0.0) (`self.PlayerCharacter`) (`KismetMathLibrary.RandomFloatInRange` 75.0 150.0)
      (:`OnSuccess`
        _)
      (:`OnFail`
        _))
    (`KismetSystemLibrary.Delay` (`KismetMathLibrary.RandomFloatInRange` 3.0 6.0))
    (`self.Follow Player`)))

(event `submerge`
  (bind (_returnvalue_x _returnvalue_y _returnvalue_z) (`KismetMathLibrary.BreakVector` (`self.K2_GetActorLocation`)))
  (`PrimitiveComponent.SetCollisionEnabled` (`self.CapsuleComponent`) "NoCollision")
  (`PrimitiveComponent.SetCollisionEnabled` (`self.Mesh`) "NoCollision")
  (set `self.ZValueTemp` _returnvalue_z)
  (bind (_direction _delta) (`Timeline|sink`)
    (:`Update`
      (`self.K2_SetActorLocation` (`KismetMathLibrary.MakeVector` _returnvalue_x _returnvalue_y (- (`self.ZValueTemp`) (* _delta 30.0))) false true))
    (:`Finished`
      (`self.K2_DestroyActor`))))

(fn `IsCharacterDead`
  (returns (IsCharacterDead :type Boolean))
  (return (`self.IsDead`)))

(fn `IsCharacterSad`
  (returns (IsCharacterSad :type Boolean))
  (return (`self.IsSad`)))

(fn `UserConstructionScript`)