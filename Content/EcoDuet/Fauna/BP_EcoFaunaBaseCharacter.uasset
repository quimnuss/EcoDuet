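; Base character Blueprint for EcoDuet fauna that wanders continuously around the level.
; On BeginPlay it caches the first actor of ElderClass as Elder, if one exists, then starts RoamAround.
; RoamAround uses AI MoveTo toward a random reachable point within Radius of its current location, then re-calls itself after a short random pause, whether the move succeeds or fails.
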(event `self.ReceiveBeginPlay`
  (`|ExecutionSequence`
    (:`then_0`
      (bind _returnvalue (`GameplayStatics.GetActorOfClass` (`self.ElderClass`)))
      (`/Engine/EditorBlueprintResources/StandardMacros.IsValid` _returnvalue
        (:`Is Valid`
          (set `self.Elder` _returnvalue))))
    (:`then_1`
      (`self.RoamAround`))))

(event `RoamAround`
  (`|AIMoveTo` self (`NavigationSystemV1.K2_GetRandomReachablePointInRadius` (`self.K2_GetActorLocation`) (`self.Radius`) null null) null 120.0
    (:`OnSuccess`
      _)
    (:`OnFail`
      _))
  (`KismetSystemLibrary.Delay` (`KismetMathLibrary.RandomFloatInRange` 1.5 4.0))
  (`self.RoamAround`))

(fn `UserConstructionScript`)