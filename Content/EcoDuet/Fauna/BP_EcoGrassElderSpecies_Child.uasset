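; Grass elder species fauna Blueprint that spawns and tracks its offspring for the ecology system.
; SpawnChildren places scaled-down ChildrenClass actors at random navigable points around itself and stores them in EcoChildren.
; AddEcoFaunaChild validates and registers a given child, then increments the Z channel of EcologyDensities on EcoGameModeHome, which SpawnChildren leaves untouched.
; Its event graph holds only disabled stubs, and construction defers to the parent.
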(fn `AddEcoFaunaChild`
  (params (NewChild :type "Actor Object Reference"))
  (bind _aseco_game_mode_home (cast `EcoGameModeHome` (`GameplayStatics.GetGameMode`) :!pure true))
  (bind (_ecologydensities_x _ecologydensities_y _ecologydensities_z _ecologydensities_w) (`KismetMathLibrary.BreakVector4` (`EcoGameModeHome.EcologyDensities` _aseco_game_mode_home)))
  (bind _isvalidecochild (`self.IsValidEcoChild` NewChild))
  (if _isvalidecochild
    (`KismetArrayLibrary.Array_Add` (`self.EcoChildren`) NewChild)
    (set `EcoGameModeHome.EcologyDensities` (`KismetMathLibrary.MakeVector4` _ecologydensities_x _ecologydensities_y (+ _ecologydensities_z 1.0) _ecologydensities_w) _aseco_game_mode_home)))

(fn `SpawnChildren`
  (params (NumChildren :type Integer))
  (for _ (range (+ NumChildren 1))
    (bind _randomlocation (`NavigationSystemV1.K2_GetRandomLocationInNavigableRadius` (`self.K2_GetActorLocation`) 1000.0 null null))
    (bind _returnvalue (`|SpawnActorFromClass` (`self.Children Class`) (`KismetMathLibrary.MakeTransform` _randomlocation (struct) (0.2 0.2 0.2)) "AdjustIfPossibleButAlwaysSpawn" "OverrideRootScale" null self))
    (`KismetArrayLibrary.Array_Add` (`self.EcoChildren`) _returnvalue)))

(fn `UserConstructionScript`
  (`parent.UserConstructionScript`))