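; Elder species actor for EcoDuet fauna that manages a population of child actors of one class.
; At BeginPlay it collects all existing actors of that class, and an event registers additional children.
; SpawnChildrenLogic compares the count to a rounded-up density, spawning children at its own transform or culling the newest through damage rather than direct destruction.
; It also offers a class-check helper and a placeholder virtual AddEcoFaunaChild for overriding.
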(event `self.ReceiveBeginPlay`
  (`parent.ReceiveBeginPlay`)
  (bind _outactors (`GameplayStatics.GetAllActorsOfClass` (`self.Children Class`)))
  (set `self.EcoChildren` _outactors))

(event `AddChildrenPlayer`
  (params (NewChild :type "Actor Object Reference"))
  (`KismetArrayLibrary.Array_Add` (`self.EcoChildren`) NewChild))

(fn `AddEcoFaunaChild`
  (params (NewChild :type "Actor Object Reference"))
  ;[1 1 1] virtual
  (`KismetSystemLibrary.PrintText` "! Called virtual function"))

(fn `DamageArrayActors`
  (params (TargetLength :type Integer) (Array :type "Array of Actor Object Reference"))
  (bind _returnvalue (`KismetArrayLibrary.Array_LastIndex` Array))
  (while (> (`KismetArrayLibrary.Array_Length` Array) TargetLength)
    (`GameplayStatics.ApplyDamage` (`|GetArrayItem` Array _returnvalue) 100.0 null self)
    (`KismetArrayLibrary.Array_Remove` Array _returnvalue)))

(fn `DestroyArrayItems`
  (params (TargetLength :type Integer) (Array :type "Array of Actor Object Reference"))
  (bind _returnvalue (`KismetArrayLibrary.Array_LastIndex` Array))
  (while (> (`KismetArrayLibrary.Array_Length` Array) TargetLength)
    (`self.K2_DestroyActor` (`|GetArrayItem` Array _returnvalue))
    (`KismetArrayLibrary.Array_Remove` Array _returnvalue)))

(fn `IsValidEcoChild`
  (params (EcoChild :type "Actor Object Reference"))
  (returns (IsValidEcoChild :type Boolean))
  (bind _returnvalue (`GameplayStatics.GetObjectClass` EcoChild))
  (bind _children_class (`self.Children Class`))
  (bind _returnvalue_2 (== _returnvalue _children_class))
  (if (not _returnvalue_2)
    (`KismetSystemLibrary.PrintText` (`|FormatText` "New actuor {new actor class} is not of class {child class}" (`KismetSystemLibrary.GetClassDisplayName` _children_class) (`KismetSystemLibrary.GetClassDisplayName` _returnvalue))))
  (return _returnvalue_2))

(fn `KillChildren`
  (params (NumChildren :type Integer))
  (locals (TargetLenght :type Integer))
  (bind _ecochildren (`self.EcoChildren`))
  (bind _output_get (set `local.TargetLenght` (- (`KismetArrayLibrary.Array_Length` _ecochildren) NumChildren)))
  (`self.DamageArrayActors` _output_get _ecochildren))

(fn `SpawnChildren`
  (params (NumChildren :type Integer))
  (for _ (range (+ NumChildren 1))
    (bind _returnvalue (`|SpawnActorFromClass` (`self.Children Class`) (`self.GetTransform` self) "AdjustIfPossibleButAlwaysSpawn" "OverrideRootScale" null self))
    (`KismetArrayLibrary.Array_Add` (`self.EcoChildren`) _returnvalue)))

(fn `SpawnChildrenLogic`
  (params (NewDensity :type "Float (double-precision)"))
  (bind _returnvalue (- (`KismetMathLibrary.FCeil` NewDensity) (`KismetArrayLibrary.Array_Length` (`self.EcoChildren`))))
  (if (== _returnvalue 0)
    _
    (elif (> _returnvalue 0)
      (`self.SpawnChildren` _returnvalue)
      (else
        (bind _result (`/Engine/EditorBlueprintResources/StandardMacros.NegateInt` _returnvalue)
          (:`  `
            (`self.KillChildren` _result)))))))

(fn `UserConstructionScript`
  (`parent.UserConstructionScript`))