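; Child pig fauna character in EcoDuet that grunts periodically and dies when damaged.
; A looping timer started on BeginPlay plays a grunt sound at the pig's location.
; Any damage calls Die directly, with an elder-species check on the damage causer left unconnected.
; Die disables movement, plays a shriek and death animation, then sets a short lifespan to remove the actor.
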(event `self.ReceiveBeginPlay`
  (`parent.ReceiveBeginPlay`)
  (bind _returnvalue (`KismetSystemLibrary.K2_SetTimerDelegate` (delegate `oink`) 11.0 true))
  (set `self.OinkTimer` _returnvalue))

(event `oink`
  (`GameplayStatics.PlaySoundAtLocation` "/Game/EcoDuet/Media/Fauna/pig-grunt.pig-grunt" (`self.K2_GetActorLocation`) (struct) 0.4 1.0 0.0 null null null null))

(event `Die`
  (`CharacterMovementComponent.DisableMovement` (`self.CharacterMovement`))
  (`GameplayStatics.PlaySoundAtLocation` "/Game/EcoDuet/Media/Fauna/pig-shriek.pig-shriek" (`self.K2_GetActorLocation`) (struct) 0.4 1.0 0.0 null null null null)
  (`SkeletalMeshComponent.PlayAnimation` (`self.Mesh`) "/Game/AnimalVarietyPack/Pig/Animations/ANIM_Pig_Death.ANIM_Pig_Death" false)
  (`self.SetLifeSpan` 5.0))

(event `self.ReceiveAnyDamage`
  (params (Damage :type "Float (single-precision)") (DamageType :type "DamageType Object Reference") (InstigatedBy :type "Controller Object Reference") (DamageCauser :type "Actor Object Reference"))
  (`self.Die`))

(fn `UserConstructionScript`
  (`parent.UserConstructionScript`))