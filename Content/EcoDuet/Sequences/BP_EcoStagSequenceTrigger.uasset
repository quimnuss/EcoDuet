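; Box trigger that plays the stag level sequence cutscene, then reveals the level door.
; BeginPlay creates the sequence player, caches "Follower"-tagged eco characters and hides the first BP_EcoDoor found.
; Character overlap changes input mode, disables movement for that character and followers, and plays the sequence.
; On finish it restores game input and walking, shows the door and sets the played flag that blocks later triggers.
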(event `self.ReceiveBeginPlay`
  (bind (_outactor _returnvalue) (`LevelSequencePlayer.CreateLevelSequencePlayer` "/Game/EcoDuet/Sequences/EcoStagSequence.EcoStagSequence"))
  (set `self.StagCutscene` _returnvalue)
  (bind _outactors (`GameplayStatics.GetAllActorsOfClassWithTag` "/Game/EcoDuet/Player/BP_EcoSimpleCharacter.BP_EcoSimpleCharacter_C" "Follower"))
  (set `self.Followers` _outactors)
  (bind _returnvalue_2 (`GameplayStatics.GetActorOfClass` "/Game/EcoDuet/Actors/doors/BP_EcoDoor.BP_EcoDoor_C"))
  (bind _output_get (set `self.LevelDoor` _returnvalue_2))
  (`SceneComponent.SetVisibility` (`/Game/EcoDuet/Actors/doors/BP_EcoDoor.DefaultSceneRoot` _output_get) false true))

(event `self.Box.OnComponentBeginOverlap`
  (params (OverlappedComponent :type "PrimitiveComponent Object Reference") (OtherActor :type "Actor Object Reference") (OtherComp :type "PrimitiveComponent Object Reference") (OtherBodyIndex :type Integer) (bFromSweep :type Boolean) (SweepResult :type "HitResult Structure (by ref)"))
  (bind _returnvalue (`GameplayStatics.GetPlayerController` 0))
  (bind _stagcutscene (`self.StagCutscene`))
  (if (not (`self.StagSequencePlayed`))
    (bind _ascharacter (cast `Character` OtherActor))
    (set `self.As Character` _ascharacter)
    (`WidgetBlueprintLibrary.SetInputMode_UIOnlyEx` _returnvalue null "DoNotLock" true)
    (`WidgetBlueprintLibrary.SetInputMode_GameAndUIEx` _returnvalue null "DoNotLock" true true)
    (`CharacterMovementComponent.DisableMovement` (`Character.CharacterMovement` _ascharacter))
    (for _array_element (`self.Followers`)
      (`CharacterMovementComponent.DisableMovement` (`Character.CharacterMovement` _array_element)))
    (`MovieSceneSequencePlayer.Play` _stagcutscene)
    (add `MovieSceneSequencePlayer.OnFinished` _stagcutscene (delegate `EnableMovement`))))

(event `EnableMovement`
  (`WidgetBlueprintLibrary.SetInputMode_GameOnly` (`GameplayStatics.GetPlayerController` 0) true)
  (`CharacterMovementComponent.SetMovementMode` (`Character.CharacterMovement` (`self.As Character`)) "MOVE_Walking" 0)
  (for _array_element (`self.Followers`)
    (`CharacterMovementComponent.SetMovementMode` (`Character.CharacterMovement` _array_element) "MOVE_Walking" 0))
  (`SceneComponent.SetVisibility` (`/Game/EcoDuet/Actors/doors/BP_EcoDoor.DefaultSceneRoot` (`self.LevelDoor`)) true true)
  (set `self.StagSequencePlayed` true))

(fn `UserConstructionScript`)