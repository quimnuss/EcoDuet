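; Short-lived compost actor in EcoDuet that applies a GLV modifier to a nearby elder tree.
; A BeginPlay timer assumes it has stopped moving shortly before its lifespan ends, then switches the box to overlap all channels.
; It takes the first elder static species in CompostArea and, if that accepts GLVMod, spawns a BP_EcoGLVModifier owned by the tree at its transform.
; If the tree refuses the modifier, the compost destroys itself immediately.
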(event `self.ReceiveBeginPlay`
  (`self.SetLifeSpan` 5.0)
  (`KismetSystemLibrary.K2_SetTimerDelegate` (delegate `AssumeStoppedMoving`) 4.0))

(event `AssumeStoppedMoving`
  (`PrimitiveComponent.SetCollisionResponseToAllChannels` (`self.Box`) "ECR_Overlap")
  (`self.CompostNearTrees`))

(fn `CompostNearTrees`
  (bind _overlappingactors (`PrimitiveComponent.GetOverlappingActors` (`self.CompostArea`) "/Game/EcoDuet/Fauna/BP_EcoElderStaticSpecies_Child.BP_EcoElderStaticSpecies_Child_C"))
  (bind _output (`|GetArrayItem` _overlappingactors))
  (if (`KismetArrayLibrary.Array_IsNotEmpty` _overlappingactors)
    (bind _asbp_eco_elder_base_species (cast `/Game/EcoDuet/Fauna/BP_EcoElderBaseSpecies` _output))
    (bind _glvmodifierapplyable (`/Game/EcoDuet/Fauna/BP_EcoElderBaseSpecies.CanApplyGLVModifier` _asbp_eco_elder_base_species (`self.GLVMod`)))
    (if _glvmodifierapplyable
      (`|SpawnActorFromClass` "/Game/EcoDuet/Actors/BP_EcoGLVModifier.BP_EcoGLVModifier_C" (`self.GetTransform` _output) "AdjustIfPossibleButAlwaysSpawn" "MultiplyWithRoot" _output (`self.GLVMod`) 10.0 null)
      (else
        (`self.K2_DestroyActor`)))))

(fn `UserConstructionScript`)