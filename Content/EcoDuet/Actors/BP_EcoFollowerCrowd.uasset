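; BP_EcoFollowerCrowd is an EcoDuet actor that starts a crowd of tagged BP_Follower actors following at level start.
; After a delay on BeginPlay, it stores player 0's BP_EcoSimpleCharacter in Players, then gathers every follower tagged "Follower".
; After another short delay it calls FollowPlayer on each one, without passing a target.
; Timing relies on fixed delays, and an alternative tag-based player lookup is left unconnected.
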(event `self.ReceiveBeginPlay`
  ;[1 1 1] switch to callbacks
  (`KismetSystemLibrary.Delay` 1.0)
  (`KismetArrayLibrary.Array_Add` (`self.Players`) (cast `/Game/EcoDuet/Player/BP_EcoSimpleCharacter` (`GameplayStatics.GetPlayerCharacter` 0) :!pure true))
  (bind _outactors (`GameplayStatics.GetAllActorsOfClassWithTag` "/Game/EcoDuet/Fauna/BP_Follower.BP_Follower_C" "Follower"))
  (bind _output_get (set `self.Followers` _outactors))
  (`KismetSystemLibrary.Delay` 0.2)
  (for _array_element _output_get
    (`/Game/EcoDuet/Fauna/BP_Follower.Follow Player` _array_element)))

(fn `UserConstructionScript`)