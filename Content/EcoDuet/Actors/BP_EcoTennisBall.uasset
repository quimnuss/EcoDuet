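; Tennis ball actor for EcoDuet that tracks which of the two character types touched it last.
; When its physics sphere hits a Koiko child character or another Eco character, the ball's material turns yellow or blue respectively and ScorePlayer records that side.
; CenterTennisBall returns it to the location saved at BeginPlay, switching physics off around the teleport.
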(event `self.ReceiveBeginPlay`
  (set `self.InitialLocation` (`self.K2_GetActorLocation`)))

(event `self.Sphere.OnComponentHit`
  (params (HitComponent :type "PrimitiveComponent Object Reference") (OtherActor :type "Actor Object Reference") (OtherComp :type "PrimitiveComponent Object Reference") (NormalImpulse :type "Vector Structure") (Hit :type "HitResult Structure (by ref)"))
  (bind _ball (`self.Ball`))
  (bind _aseco_duet_character (cast `EcoDuetCharacter` OtherActor))
  (cast `/Game/EcoDuet/Player/BP_EcoKoikoCharacter_Child` _aseco_duet_character
    (:`then`
      (`PrimitiveComponent.SetMaterial` _ball 0 "/Game/PhotoR_Backgrounds/Meshes/template_yellow.template_yellow")
      (set `self.ScorePlayer` 0))
    (:`CastFailed`
      (cast `/Game/EcoDuet/Player/BP_EcoCharacter` _aseco_duet_character)
      (`PrimitiveComponent.SetMaterial` _ball 0 "/AnimationSharing/AnimSharingBlue.AnimSharingBlue")
      (set `self.ScorePlayer` 1))))

(event `CenterTennisBall`
  (bind _sphere (`self.Sphere`))
  (`PrimitiveComponent.SetSimulatePhysics` _sphere false)
  (`self.K2_SetActorLocation` (`self.InitialLocation`) false true)
  (`PrimitiveComponent.SetSimulatePhysics` _sphere true))

(fn `UserConstructionScript`)