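; BP_EcoDrop is a spinning collectible cube that grants seed abilities to the BP_EcoCharacter overlapping it.
; A drop-type-to-material map sets its look on BeginPlay or through SetDrop.
; CheckIsSeed detects seeds by matching the drop enum name against "Elder{species}Seed" for each species.
; On pickup it fires Caught, destroys itself and adds the seed ability; non-seed abilities are only a TODO print.
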(event `self.ReceiveBeginPlay`
  (bind _droptype (`self.DropType`))
  (bind (_value _returnvalue) (`BlueprintMapLibrary.Map_Find` (`self.EcoDropMaterialMap`) _droptype))
  (if _returnvalue
    (`PrimitiveComponent.SetMaterial` (`self.DropCube`) 0 _value))
  (bind (_seedfound _seedspecies) (`self.CheckIsSeed` _droptype))
  (set `self.IsSeed` _seedfound)
  (set `self.Seed Species` _seedspecies))

(event `self.ReceiveTick`
  (params (DeltaSeconds :type "Float (single-precision)"))
  (`SceneComponent.K2_AddLocalRotation` (`self.DropCube`) (`KismetMathLibrary.MakeRotator` 0.0 0.0 (* DeltaSeconds (`self.RotationSpeed`))) false false))

(event `self.ActivationBox.OnComponentBeginOverlap`
  (params (OverlappedComponent :type "PrimitiveComponent Object Reference") (OtherActor :type "Actor Object Reference") (OtherComp :type "PrimitiveComponent Object Reference") (OtherBodyIndex :type Integer) (bFromSweep :type Boolean) (SweepResult :type "HitResult Structure (by ref)"))
  (bind _asbp_eco_character (cast `/Game/EcoDuet/Player/BP_EcoCharacter` OtherActor))
  (`self.Caught`)
  (`self.K2_DestroyActor`)
  (if (`self.IsSeed`)
    (`/Game/EcoDuet/Player/BP_EcoCharacter.AddSeedAbility` _asbp_eco_character (`self.Seed Species`))
    (else
      (`KismetSystemLibrary.PrintText` "TODO habilities"))))

(fn `CheckIsSeed`
  (params (DropType :type "/Game/EcoDuet/Actors/EcoDropEnum Enum" :default "NewEnumerator0"))
  (returns (SeedFound :type Boolean) (SeedSpecies :type "EEcoSpeciesType Enum"))
  (bind _enumvalue (foreach `EEcoSpeciesType` false)
    (:`LoopBody`
      (if (== (`KismetTextLibrary.Conv_TextToString` (`|FormatText` "Elder{species}Seed" (`|GetEnumeratorNameAsString` _enumvalue))) (`|GetEnumeratorNameAsString` DropType))
        (return true _enumvalue)))
    (:`then`
      (return false "EcoGrass"))))

(fn `SetDrop`
  (params (EcoDropType :type "/Game/EcoDuet/Actors/EcoDropEnum Enum" :default "NewEnumerator0"))
  (bind (_value _returnvalue) (`BlueprintMapLibrary.Map_Find` (`self.EcoDropMaterialMap`) EcoDropType))
  (if _returnvalue
    (`PrimitiveComponent.SetMaterial` (`self.DropCube`) 0 _value)
    (bind (_seedfound _seedspecies) (`self.CheckIsSeed` EcoDropType))
    (set `self.IsSeed` _seedfound)
    (set `self.Seed Species` _seedspecies)
    (else
      (`KismetSystemLibrary.PrintText` (`|FormatText` "Drop type {type} not found" (`|GetEnumeratorNameAsString` EcoDropType))))))

(fn `UserConstructionScript`
  (bind (_seedfound _seedspecies) (`self.CheckIsSeed` (`self.DropType`)))
  (set `self.IsSeed` _seedfound)
  (set `self.Seed Species` _seedspecies))