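; BP_EcoInteractionCube is an EcoDuet actor for a selectable interaction cube that signals its state through two spotlights.
; Select and Deselect set an IsSelected flag and show or hide both lights to match.
; ColorLights tints both lights green for zero or positive values and red for negative ones.
; Its event graph and construction script are empty, so it relies on external callers to invoke these functions.
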(fn `ColorLights`
  (params (NewValue :type "Float (double-precision)"))
  (bind _linearcolor (make `LinearColor` 1.0))
  (bind _linearcolor_2 (make `LinearColor` 0.0 1.0))
  (bind _spotlight1 (`self.SpotLight1`))
  (bind _spotlight (`self.SpotLight`))
  (if (>= NewValue 0.0)
    (`LightComponent.SetLightColor` _spotlight _linearcolor_2 true)
    (`LightComponent.SetLightColor` _spotlight1 _linearcolor_2 true)
    (else
      (`LightComponent.SetLightColor` _spotlight _linearcolor true)
      (`LightComponent.SetLightColor` _spotlight1 _linearcolor true))))

(fn `Deselect`
  (bind _output_get (set `self.IsSelected` false))
  (`SceneComponent.SetVisibility` (`self.SpotLight`) _output_get false)
  (`SceneComponent.SetVisibility` (`self.SpotLight1`) _output_get false))

(fn `Select`
  (bind _output_get (set `self.IsSelected` true))
  (`SceneComponent.SetVisibility` (`self.SpotLight`) _output_get false)
  (`SceneComponent.SetVisibility` (`self.SpotLight1`) _output_get false))

(fn `UserConstructionScript`)