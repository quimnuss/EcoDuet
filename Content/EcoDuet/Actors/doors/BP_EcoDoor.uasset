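; BP_EcoDoor is an interactable door that leads to another level through a portal.
; Interact, when the door is openable, reveals the Portal and swings the Door open with a timeline, which reverses after a short retriggerable delay and hides the Portal once closed.
; An Eco character or simple character overlapping the Portal saves persistent data through the game instance, then opens LevelName if one is set.
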(event `OpenDoor`
  (bind _portal (`self.Portal`))
  (`SceneComponent.SetVisibility` _portal true false)
  (bind (_direction _dooropenfloat) (`Timeline|OpenDoorTimeline` :!label _label)
    (:`Update`
      (`SceneComponent.K2_SetRelativeRotation` (`self.Door`) (`KismetMathLibrary.MakeRotator` 0.0 0.0 (`KismetMathLibrary.Lerp` 0.0 90.0 _dooropenfloat)) false false))
    (:`Finished`
      (switch `ETimelineDirection` _direction
        (:`Forward`
          (`KismetSystemLibrary.RetriggerableDelay` 2.0)
          (`self.CloseDoor`))
        (:`Backward`
          (`SceneComponent.SetVisibility` _portal false false))))))

(event `CloseDoor`
  (goto _label :!via `Reverse`))

(event `/Game/EcoDuet/Actors/BPI_EcoInteractable.Interact`
  (if (`self.IsOpenable`)
    (`self.OpenDoor`)))

(event `self.Portal.OnComponentBeginOverlap`
  (params (OverlappedComponent :type "PrimitiveComponent Object Reference") (OtherActor :type "Actor Object Reference") (OtherComp :type "PrimitiveComponent Object Reference") (OtherBodyIndex :type Integer) (bFromSweep :type Boolean) (SweepResult :type "HitResult Structure (by ref)"))
  (bind _level_name (`self.Level Name`))
  (cast `/Game/EcoDuet/Player/BP_EcoCharacter` OtherActor
    (:`then`
      _)
    (:`CastFailed`
      (cast `/Game/EcoDuet/Player/BP_EcoSimpleCharacter` OtherActor)))
  (`/Game/EcoDuet/GameLogic/Bp_EcoGameInstance.SavePersistentData` (cast `/Game/EcoDuet/GameLogic/Bp_EcoGameInstance` (`GameplayStatics.GetGameInstance`) :!pure true))
  (if (!= _level_name "None")
    (`GameplayStatics.OpenLevel` _level_name)))

(fn `UserConstructionScript`
  (`SceneComponent.SetVisibility` (`self.Portal`) false false))