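; BP_EcoTennisWall is a wall that reacts to BP_EcoTennisBall and tracks a ScoreOwner.
; On hit, it applies a scaled-down normal impulse to the ball and takes the ball's ScorePlayer as owner.
; The cube flashes red briefly, then adopts the ball's material.
; Box overlap begin and end also toggle the cube between red and blue and set the owner to 0 or 1.
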(event `self.Box.OnComponentBeginOverlap`
  (params (OverlappedComponent :type "PrimitiveComponent Object Reference") (OtherActor :type "Actor Object Reference") (OtherComp :type "PrimitiveComponent Object Reference") (OtherBodyIndex :type Integer) (bFromSweep :type Boolean) (SweepResult :type "HitResult Structure (by ref)"))
  (cast `/Game/EcoDuet/Actors/BP_EcoTennisBall` OtherActor)
  (`PrimitiveComponent.SetMaterial` (`self.Cube`) 0 "/AnimationSharing/AnimSharingRed.AnimSharingRed")
  (set `self.ScoreOwner` 0))

(event `self.Box.OnComponentEndOverlap`
  (params (OverlappedComponent :type "PrimitiveComponent Object Reference") (OtherActor :type "Actor Object Reference") (OtherComp :type "PrimitiveComponent Object Reference") (OtherBodyIndex :type Integer))
  (cast `/Game/EcoDuet/Actors/BP_EcoTennisBall` OtherActor)
  (`PrimitiveComponent.SetMaterial` (`self.Cube`) 0 "/AnimationSharing/AnimSharingBlue.AnimSharingBlue")
  (set `self.ScoreOwner` 1))

(event `self.Box.OnComponentHit`
  (params (HitComponent :type "PrimitiveComponent Object Reference") (OtherActor :type "Actor Object Reference") (OtherComp :type "PrimitiveComponent Object Reference") (NormalImpulse :type "Vector Structure") (Hit :type "HitResult Structure (by ref)"))
  (bind _asbp_eco_tennis_ball (cast `/Game/EcoDuet/Actors/BP_EcoTennisBall` OtherActor))
  (`PrimitiveComponent.AddImpulse` (`/Game/EcoDuet/Actors/BP_EcoTennisBall.Ball` _asbp_eco_tennis_ball) (/ NormalImpulse 1.5) "None" false)
  (set `self.ScoreOwner` (`/Game/EcoDuet/Actors/BP_EcoTennisBall.ScorePlayer` _asbp_eco_tennis_ball))
  (`PrimitiveComponent.SetMaterial` (`self.Cube`) 0 "/AnimationSharing/AnimSharingRed.AnimSharingRed")
  (set `self.LastMaterial` (`PrimitiveComponent.GetMaterial` (`/Game/EcoDuet/Actors/BP_EcoTennisBall.Ball` _asbp_eco_tennis_ball) 0))
  (`KismetSystemLibrary.Delay` 0.05)
  (`PrimitiveComponent.SetMaterial` (`self.Cube`) 0 (`self.LastMaterial`)))

(fn `UserConstructionScript`)