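; BP_EcoTutorialMonkey is a tutorial actor that shows text for the current tutorial step when something comes near it.
; On BeginPlay it binds to the step-change event of BP_EcoGameModeTutorial.
; Each change looks up TutorialStateMap by the step, wrapped by map length, and sets the text on its BP_EcoTextActor child actor.
; Sphere overlap begin and end show and hide that child actor component, without filtering the overlapping actor.
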(event `self.ReceiveBeginPlay`
  (add `/Game/EcoDuet/GameLogic/BP_EcoGameModeTutorial.TutorialStepChange` (cast `/Game/EcoDuet/GameLogic/BP_EcoGameModeTutorial` (`GameplayStatics.GetGameMode`) :!pure true) (delegate `UpdateTutorialStep`)))

(event `UpdateTutorialStep`
  (bind _tutorialstatemap (`self.TutorialStateMap`))
  (`TextRenderComponent.K2_SetText` (`/Game/EcoDuet/Actors/BP_EcoTextActor.TutorialText` (cast `/Game/EcoDuet/Actors/BP_EcoTextActor` (`ChildActorComponent.ChildActor` (`self.ChildActor`)) :!pure true)) (`|GetArrayItem` _tutorialstatemap (mod (`/Game/EcoDuet/GameLogic/BP_EcoGameModeTutorial.TutorialStep` (cast `/Game/EcoDuet/GameLogic/BP_EcoGameModeTutorial` (`GameplayStatics.GetGameMode`) :!pure true)) (`KismetArrayLibrary.Array_Length` _tutorialstatemap)))))

(event `self.Sphere.OnComponentBeginOverlap`
  (params (OverlappedComponent :type "PrimitiveComponent Object Reference") (OtherActor :type "Actor Object Reference") (OtherComp :type "PrimitiveComponent Object Reference") (OtherBodyIndex :type Integer) (bFromSweep :type Boolean) (SweepResult :type "HitResult Structure (by ref)"))
  (`SceneComponent.SetVisibility` (`self.ChildActor`) true false))

(event `self.Sphere.OnComponentEndOverlap`
  (params (OverlappedComponent :type "PrimitiveComponent Object Reference") (OtherActor :type "Actor Object Reference") (OtherComp :type "PrimitiveComponent Object Reference") (OtherBodyIndex :type Integer))
  (`SceneComponent.SetVisibility` (`self.ChildActor`) false false))

(fn `UserConstructionScript`)