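; BP_EcoGLVModifier is a temporary actor that applies a timed buff or debuff to an Elder species' GLV.
; On BeginPlay it casts its owner to BP_EcoElderBaseSpecies, attaches itself to that Elder and adds its GLV modifier.
; A one-shot timer set to the buff time then reverts the modifier and destroys the actor.
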(event `self.ReceiveBeginPlay`
  (bind _asbp_eco_elder_base_species (cast `/Game/EcoDuet/Fauna/BP_EcoElderBaseSpecies` (`self.GetOwner`)))
  (bind _output_get (set `self.Elder` _asbp_eco_elder_base_species))
  (`self.K2_AttachToActor` _output_get "None" "SnapToTarget" "KeepRelative" "KeepRelative")
  (`/Game/EcoDuet/Fauna/BP_EcoElderBaseSpecies.AddGLVModifier` (`self.Elder`) (`self.GLVMod`))
  (`KismetSystemLibrary.K2_SetTimerDelegate` (delegate `RevertBuffDebuff`) (`self.BuffTime`)))

(event `RevertBuffDebuff`
  (`/Game/EcoDuet/Fauna/BP_EcoElderBaseSpecies.RevertGLVModifier` (`self.Elder`) (`self.GLVMod`))
  (`self.K2_DestroyActor`))

(fn `UserConstructionScript`)