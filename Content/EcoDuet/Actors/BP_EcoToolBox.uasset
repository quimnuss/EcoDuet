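; BP_EcoToolBox is a tool box actor that shows an eco species selection as a spinning mini cube.
; SwitchElderTool steps CurrentSpecies through the species enum, wrapping around by entry count, and updates the cube's material from EcoElderMaterialMap.
; BeginPlay applies the grass material without setting CurrentSpecies, and Tick rotates the cube by a fixed step each frame, independent of delta time.
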(event `self.ReceiveBeginPlay`
  (`self.SetCubeMaterial` "EcoGrass"))

(event `self.ReceiveTick`
  (params (DeltaSeconds :type "Float (single-precision)"))
  (`SceneComponent.K2_AddLocalRotation` (`self.EcoMiniCube`) (struct :`Yaw` 5.0) false false))

(event `SwitchElderTool`
  (bind _result (`/Engine/EditorBlueprintResources/StandardMacros.IncrementInt` (`KismetMathLibrary.Conv_ByteToInt` (`self.CurrentSpecies`)))
    (:`  `
      (bind _output_get (set `self.CurrentSpecies` (cast `EEcoSpeciesType` (`KismetMathLibrary.Conv_IntToByte` (mod _result (enumcount `EEcoSpeciesType`))))))
      (`self.SetCubeMaterial` _output_get))))

(fn `SetCubeMaterial`
  (params (EcoSpecies :type "EEcoSpeciesType Enum" :default "EcoFox"))
  (`PrimitiveComponent.SetMaterial` (`self.EcoMiniCube`) 0 (`BlueprintMapLibrary.Map_Find` (`self.EcoElderMaterialMap`) EcoSpecies)))

(fn `UserConstructionScript`)