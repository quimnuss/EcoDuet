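; BP_EcoGameModeHomeSurvival is a game mode for a home survival scenario that ends when the ecosystem dies.
; A looping 20-second timer started on BeginPlay calls CountExtinctSpecies and stores the result as EcosystemIsDead.
; Once that is true, it clears the timer, syncs the menu's eco message and shows the menu.
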(event `self.ReceiveBeginPlay`
  (`parent.ReceiveBeginPlay`)
  (bind _returnvalue (`KismetSystemLibrary.K2_SetTimerDelegate` (delegate `CustomEvent`) 20.0 true))
  (set `self.IsEcosystemDeadTimer` _returnvalue))

(event `CustomEvent`
  (bind _ecosystemisdead (`self.CountExtinctSpecies`))
  (bind _output_get (set `self.Ecosystem Is Dead` _ecosystemisdead))
  (if _output_get
    (`KismetSystemLibrary.K2_ClearAndInvalidateTimerHandle` (`self.IsEcosystemDeadTimer`))
    (`/Game/EcoDuet/UI/EcoMenuWidget.SyncEcoMessage` (`self.Menu`))
    (`self.ShowMenu`)))

(fn `UserConstructionScript`
  (`parent.UserConstructionScript`))