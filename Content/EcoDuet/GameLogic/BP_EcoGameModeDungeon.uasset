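; BP_EcoGameModeDungeon is the game mode for EcoDuet's dungeon, setting up input for two local players.
; On BeginPlay it runs the parent logic, then fetches player controllers 0 and 1 as BP_EcoPlayerController.
; It adds the dungeon Enhanced Input mapping context to each at priority zero.
; A failed cast on the first controller also skips the second player's setup.
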(event `self.ReceiveBeginPlay`
  (`parent.ReceiveBeginPlay`)
  (bind _asbp_eco_player_controller (cast `/Game/EcoDuet/Player/BP_EcoPlayerController` (`GameplayStatics.GetPlayerControllerFromID` 0)))
  (message `EnhancedInputSubsystemInterface.AddMappingContext` (pcsubsystem `EnhancedInputLocalPlayerSubsystem` _asbp_eco_player_controller) "/Game/EcoDuet/Player/Input/EcoDungeonPlayerInputContext.EcoDungeonPlayerInputContext" 0 (struct))
  (bind _asbp_eco_player_controller_2 (cast `/Game/EcoDuet/Player/BP_EcoPlayerController` (`GameplayStatics.GetPlayerControllerFromID` 1)))
  (message `EnhancedInputSubsystemInterface.AddMappingContext` (pcsubsystem `EnhancedInputLocalPlayerSubsystem` _asbp_eco_player_controller_2) "/Game/EcoDuet/Player/Input/EcoDungeonPlayerInputContext.EcoDungeonPlayerInputContext" 0 (struct)))

(fn `UserConstructionScript`
  (`parent.UserConstructionScript`))