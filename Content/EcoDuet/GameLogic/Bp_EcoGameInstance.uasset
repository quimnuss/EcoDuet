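; EcoDuet game instance that holds elder species and ecologist ability data to save and restore as persistent game state.
; Saving serializes the SpeciesManager's elders on home maps only and copies Ecologist1's toolbox abilities.
; Loading re-adds elders and their densities through the home game mode, unless a one-shot flag skips it, then runs species spawning.
; Fixed delays, rather than callbacks, time the restore, which applies the saved abilities to both ecologists.
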(event `SavePersistentData`
  (bind _ecologist1 (`self.Ecologist1`))
  ;[1 1 1] TODO maybe we should always have the data here instead that only on save
  (`/Engine/EditorBlueprintResources/StandardMacros.IsValid` _ecologist1
    (:`Is Valid`
      (`self.SaveElderData`))
    (:`Is Not Valid`
      (`KismetSystemLibrary.PrintText` (`|FormatText` "[EcoGameInstance] Ecologist {ecologist} is not valid" (`KismetSystemLibrary.GetDisplayName` _ecologist1)) true true (struct :`R` 1.0 :`G` 0.133161 :`B` 0.192895 :`A` 1.0) 5.0)))
  (set `self.Available Abilities` (`/Game/EcoDuet/Actors/BP_EcoToolBox.AvailableAbilities` (`/Game/EcoDuet/Player/BP_EcoCharacter.ToolBox` _ecologist1))))

(event `LoadPersistentData`
  (bind _ecologist2 (`self.Ecologist2`))
  (bind _ecologist1 (`self.Ecologist1`))
  (bind _available_abilities (`self.Available Abilities`))
  (if (`self.IgnoreElderData`)
    (set `self.IgnoreElderData` false)
    (else
      (`KismetSystemLibrary.DelayUntilNextTick`)
      (`self.LoadElderData`)))
  (`KismetSystemLibrary.Delay` 0.2)
  (`/Engine/EditorBlueprintResources/StandardMacros.IsValid` _ecologist1
    (:`Is Valid`
      (`/Game/EcoDuet/Actors/BP_EcoToolBox.SetAbilities` (`/Game/EcoDuet/Player/BP_EcoCharacter.ToolBox` _ecologist1) _available_abilities)
      (`/Engine/EditorBlueprintResources/StandardMacros.IsValid` _ecologist2
        (:`Is Valid`
          (`/Game/EcoDuet/Actors/BP_EcoToolBox.SetAbilities` (`/Game/EcoDuet/Player/BP_EcoCharacter.ToolBox` _ecologist2) _available_abilities))))
    (:`Is Not Valid`
      (`KismetSystemLibrary.PrintText` "[EcoGameInstance] Ecologist is not valid! we need to switch to callbacks or something"))))

(event `SaveElderData`
  (bind _asbp_eco_game_mode_home (cast `/Game/EcoDuet/GameLogic/BP_EcoGameModeHome` (`GameplayStatics.GetGameMode`))
    (:`then`
      (`KismetArrayLibrary.Array_Clear` (`self.Elders`))
      (bind _values (`BlueprintMapLibrary.Map_Values` (`/Game/EcoDuet/Fauna/BP_EcoSpeciesManager.ElderMap` (`/Game/EcoDuet/GameLogic/BP_EcoGameModeHome.SpeciesManager` _asbp_eco_game_mode_home))))
      (for _array_element _values
        (bind _elderdata (`/Game/EcoDuet/Fauna/BP_EcoElderBaseSpecies.SerializeToData` _array_element))
        (`KismetArrayLibrary.Array_Add` (`self.Elders`) _elderdata)))
    (:`CastFailed`
      (`KismetSystemLibrary.PrintString` "Not a home map, ignoring elder data" :!label _label))))

(event `LoadElderData`
  (bind _asbp_eco_game_mode_home (cast `/Game/EcoDuet/GameLogic/BP_EcoGameModeHome` (`GameplayStatics.GetGameMode`))
    (:`then`
      (`KismetSystemLibrary.DelayUntilNextTick`)
      (bind _speciesmanager (`/Game/EcoDuet/GameLogic/BP_EcoGameModeHome.SpeciesManager` _asbp_eco_game_mode_home))
      (`BlueprintMapLibrary.Map_Clear` (`/Game/EcoDuet/Fauna/BP_EcoSpeciesManager.ElderMap` _speciesmanager))
      (for _array_element (`self.Elders`)
        (bind (_species _charactertransform _baseglv _modifiers _density) (break `/Game/EcoDuet/Fauna/EcoElderData` _array_element))
        ;[1 1 1] TODO move code from game mode to species manager
        (`/Game/EcoDuet/GameLogic/BP_EcoGameModeHome.AddElder` (cast `/Game/EcoDuet/GameLogic/BP_EcoGameModeHome` (`GameplayStatics.GetGameMode`) :!pure true) _species _charactertransform)
        (`BlueprintMapLibrary.Map_Add` (`/Game/EcoDuet/GameLogic/BP_EcoGameModeHome.EcologySpeciesDensitiesMap` (cast `/Game/EcoDuet/GameLogic/BP_EcoGameModeHome` (`GameplayStatics.GetGameMode`) :!pure true)) _species _density))
      (`/Game/EcoDuet/Fauna/BP_EcoSpeciesManager.SpawnSpeciesLogic` _speciesmanager))
    (:`CastFailed`
      (goto _label))))

(event `SavePlayerData`)