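; Game mode for the EcoDuet home level, setting up the species manager reference, main HUD and Enhanced Input mapping for two player controllers.
; AddElder spawns a single elder per species class from the manager's GLV defaults, raises that species' density and registers the elder with the manager.
; CountExtinctSpecies checks the density map and reports whether at most one species remains above the survival threshold.
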(event `self.ReceiveBeginPlay`
  (`parent.ReceiveBeginPlay`)
  (`|ExecutionSequence`
    (:`then_0`
      (bind _returnvalue (`GameplayStatics.GetActorOfClass` "/Game/EcoDuet/Fauna/BP_EcoSpeciesManager.BP_EcoSpeciesManager_C"))
      (set `self.SpeciesManager` _returnvalue)
      (bind _returnvalue_2 (`|CreateWidget` "/Game/EcoDuet/UI/EcoMainHUDWidget.EcoMainHUDWidget_C"))
      (bind _output_get (set `self.HUD` _returnvalue_2))
      (`UserWidget.AddToViewport` _output_get 0))
    (:`then_1`
      (bind _asbp_eco_player_controller (cast `/Game/EcoDuet/Player/BP_EcoPlayerController` (`GameplayStatics.GetPlayerControllerFromID` 0)))
      (message `EnhancedInputSubsystemInterface.AddMappingContext` (pcsubsystem `EnhancedInputLocalPlayerSubsystem` _asbp_eco_player_controller) "/Game/EcoDuet/Player/Input/EcoPlayerInputContext.EcoPlayerInputContext" 1 (struct))
      (bind _asbp_eco_player_controller_2 (cast `/Game/EcoDuet/Player/BP_EcoPlayerController` (`GameplayStatics.GetPlayerControllerFromID` 1)))
      (message `EnhancedInputSubsystemInterface.AddMappingContext` (pcsubsystem `EnhancedInputLocalPlayerSubsystem` _asbp_eco_player_controller_2) "/Game/EcoDuet/Player/Input/EcoPlayerInputContext.EcoPlayerInputContext" 1 (struct)))))

(fn `AddElder`
  (params (NewElderSpecies :type "EEcoSpeciesType Enum" :default "EcoNone") (SpawnTransform :type "Transform Structure"))
  (bind _returnvalue (`|GetEnumeratorName` NewElderSpecies))
  (bind _ecologyspeciesdensitiesmap (`self.EcologySpeciesDensitiesMap`))
  (bind (_value _returnvalue_2) (`BlueprintMapLibrary.Map_Find` _ecologyspeciesdensitiesmap NewElderSpecies))
  (bind (_value_2 _returnvalue_3) (`BlueprintMapLibrary.Map_Find` (`/Game/EcoDuet/Fauna/BP_EcoSpeciesManager.ElderDefaultsMap` (`self.SpeciesManager`)) NewElderSpecies))
  (bind _asbp_eco_elder_base_species (castclass `/Game/EcoDuet/Fauna/BP_EcoElderBaseSpecies` (`EcoElderDataAsset.SpeciesClass` _value_2) :!pure true))
  (if _returnvalue_3
    (bind _returnvalue_4 (`GameplayStatics.GetActorOfClass` _asbp_eco_elder_base_species))
    (`/Engine/EditorBlueprintResources/StandardMacros.IsValid` _returnvalue_4
      (:`Is Valid`
        (`KismetSystemLibrary.PrintText` (`|FormatText` "[BP_EcoGameModeHome] {Elder} already exists" _returnvalue)))
      (:`Is Not Valid`
        (bind _returnvalue_5 (`|SpawnActorFromClass` _asbp_eco_elder_base_species SpawnTransform "AdjustIfPossibleButAlwaysSpawn" "MultiplyWithRoot" null _value_2 null))
        (if _returnvalue_2
          (`BlueprintMapLibrary.Map_Add` _ecologyspeciesdensitiesmap NewElderSpecies (+ _value 1.0))
          (else
            (`BlueprintMapLibrary.Map_Add` _ecologyspeciesdensitiesmap NewElderSpecies 2.0)))
        (`/Game/EcoDuet/Fauna/BP_EcoSpeciesManager.AddElder` (`self.SpeciesManager`) _returnvalue_5)))
    (else
      (`KismetSystemLibrary.PrintText` (`|FormatText` "[BP_EcoGameModeHome] Species GLV Default for {Elder} not found in defaults" _returnvalue)))))

(fn `CountExtinctSpecies`
  (returns (EcosystemIsDead :type Boolean))
  (locals (NumSpeciesAlive :type Integer))
  (bind _values (`BlueprintMapLibrary.Map_Values` (`self.EcologySpeciesDensitiesMap`)))
  (for _array_element _values
    (if (>= _array_element 0.01)
      (`/Engine/EditorBlueprintResources/StandardMacros.IncrementInt` (`local.NumSpeciesAlive`))))
  (return (<= (`local.NumSpeciesAlive`) 1)))

(fn `UserConstructionScript`)