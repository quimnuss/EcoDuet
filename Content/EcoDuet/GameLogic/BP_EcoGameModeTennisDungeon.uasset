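; Game mode for a two-player tennis dungeon where score is the number of tennis walls each side owns, blue versus red.
; BeginPlay creates the HUD, gathers all tennis walls, and assigns the Koiko character as Player1 and the other character as Player2.
; A looping timer recounts wall owners, updates both HUD scores, and shows the highlight plane on the leading player, hiding both on a tie.
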(event `self.ReceiveBeginPlay`
  (`parent.ReceiveBeginPlay`)
  (`|ExecutionSequence`
    (:`then_0`
      (bind _returnvalue (`|CreateWidget` "/Game/EcoDuet/UI/EcoTennisHUDWidget.EcoTennisHUDWidget_C"))
      (bind _output_get (set `self.TennisHUD` _returnvalue))
      (`Widget.SetVisibility` _output_get "Visible")
      (`UserWidget.AddToViewport` _output_get 0))
    (:`then_1`
      (bind _outactors (`GameplayStatics.GetAllActorsOfClass` "/Game/EcoDuet/Actors/BP_EcoTennisWall.BP_EcoTennisWall_C"))
      (set `self.TennisWalls` _outactors))
    (:`then_2`
      (`KismetSystemLibrary.DelayUntilNextTick`)
      (bind _outactors_2 (`GameplayStatics.GetAllActorsOfClass` "/Game/EcoDuet/Player/BP_EcoCharacter.BP_EcoCharacter_C"))
      (for _array_element _outactors_2
        (bind _asbp_eco_koiko_character_child (cast `/Game/EcoDuet/Player/BP_EcoKoikoCharacter_Child` _array_element)
          (:`then`
            (set `self.Player1` _asbp_eco_koiko_character_child))
          (:`CastFailed`
            (set `self.Player2` _array_element)))))
    (:`then_3`
      (`KismetSystemLibrary.DelayUntilNextTick`)
      (bind _returnvalue_2 (`KismetSystemLibrary.K2_SetTimerDelegate` (delegate `TickScore`) 0.3 true))
      (set `self.ScoreTimerHandle` _returnvalue_2))))

(event `TickScore`
  (bind _tennishud (`self.TennisHUD`))
  (bind _blue_score (`self.Blue Score`))
  (bind _red_score (`self.Red Score`))
  (bind _highlightplane (`/Game/EcoDuet/Player/BP_EcoCharacter.HighlightPlane` (`self.Player1`)))
  (bind _highlightplane_2 (`/Game/EcoDuet/Player/BP_EcoCharacter.HighlightPlane` (`self.Player2`)))
  (bind (_bluescore _redscore) (`self.UpdateTennisScore`))
  (`|ExecutionSequence`
    (:`then_0`
      (bind _output_get (set `self.Blue Score` _bluescore))
      (set `/Game/EcoDuet/UI/EcoTennisHUDWidget.BlueScore` _output_get _tennishud)
      (bind _output_get_2 (set `self.Red Score` _redscore))
      (set `/Game/EcoDuet/UI/EcoTennisHUDWidget.RedScore` _output_get_2 _tennishud))
    (:`then_1`
      (`/Engine/EditorBlueprintResources/StandardMacros.IsValid` _highlightplane
        (:`Is Valid`
          (if (== _blue_score _red_score)
            (`SceneComponent.SetVisibility` _highlightplane false false)
            (`SceneComponent.SetVisibility` _highlightplane_2 false false)
            (elif (> _blue_score _red_score)
              (`SceneComponent.SetVisibility` _highlightplane true false)
              (`SceneComponent.SetVisibility` _highlightplane_2 false false)
              (else
                (`SceneComponent.SetVisibility` _highlightplane false false)
                (`SceneComponent.SetVisibility` _highlightplane_2 true false)))))))))

(fn `UpdateTennisScore`
  (returns (BlueScore :type Integer) (RedScore :type Integer))
  (locals (BlueScoreTmp :type Integer) (RedScoreTmp :type Integer))
  (for _array_element (`self.TennisWalls`)
    (switch `int` (`/Game/EcoDuet/Actors/BP_EcoTennisWall.ScoreOwner` _array_element)
      (:`0`
        (`/Engine/EditorBlueprintResources/StandardMacros.IncrementInt` (`local.BlueScoreTmp`)))
      (:`1`
        (`/Engine/EditorBlueprintResources/StandardMacros.IncrementInt` (`local.RedScoreTmp`)))))
  (return (`local.BlueScoreTmp`) (`local.RedScoreTmp`)))

(fn `UserConstructionScript`
  (`parent.UserConstructionScript`))