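; Game mode for the EcoDuet lobby, which sets up the menu and lets the displayed character be cycled.
; On BeginPlay it caches the lobby pawns and a display spot based on the PlayerStart, blends to the first tagged fixed camera and shows the lobby menu widget.
; SwapCharacters plays a sound, teleports the current pawn to the world origin and moves the next one, wrapping around, into the display spot.
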(event `self.ReceiveBeginPlay`
  (bind _returnvalue (`GameplayStatics.GetActorOfClass` "/Script/Engine.PlayerStart"))
  (bind (_returnvalue_x _returnvalue_y _returnvalue_z) (`KismetMathLibrary.BreakVector` (`self.K2_GetActorLocation` _returnvalue)))
  (set `self.EcoCharacterLocation` (`KismetMathLibrary.MakeVector` _returnvalue_x _returnvalue_y (/ _returnvalue_z 2.0)))
  (bind _outactors (`GameplayStatics.GetAllActorsOfClass` "/Game/EcoDuet/Player/EcoLobbyPawn.EcoLobbyPawn_C"))
  (set `self.EcoCharacters` _outactors)
  (bind _outactors_2 (`GameplayStatics.GetAllActorsOfClassWithTag` "/Script/Engine.CameraActor" "EcoFixedCamera"))
  (bind _output_get (set `self.EcoCameras` _outactors_2))
  (`PlayerController.SetViewTargetWithBlend` (`GameplayStatics.GetPlayerController` 0) (`|GetArrayItem` _output_get) 1.0 "VTBlend_Linear" 0.0 false)
  (bind _returnvalue_2 (`|CreateWidget` "/Game/EcoDuet/UI/EcoLobbyMenuWidget.EcoLobbyMenuWidget_C"))
  (bind _output_get_2 (set `self.LobbyMenu` _returnvalue_2))
  (`Widget.SetVisibility` _output_get_2 "Visible")
  (`UserWidget.AddToViewport` _output_get_2 0))

(event `SwapCharacters`
  (`GameplayStatics.PlaySoundAtLocation` "/Engine/VREditor/Sounds/UI/Dockable_Window_Drop.Dockable_Window_Drop" (`self.EcoCharacterLocation`) (struct) 1.0 1.0 0.0 null null null null)
  (`self.K2_SetActorLocation` (`|GetArrayItem` (`self.EcoCharacters`) (`self.CurrentCharacterIndex`)) (0.0 0.0 0.0) false false)
  (bind _result (`/Engine/EditorBlueprintResources/StandardMacros.IncrementInt` (`self.CurrentCharacterIndex`))
    (:`  `
      (bind _output_get (set `self.CurrentCharacterIndex` (mod _result (`KismetArrayLibrary.Array_Length` (`self.EcoCharacters`)))))
      (`self.K2_SetActorLocation` (`|GetArrayItem` (`self.EcoCharacters`) _output_get) (`self.EcoCharacterLocation`) false false))))

(fn `UserConstructionScript`)