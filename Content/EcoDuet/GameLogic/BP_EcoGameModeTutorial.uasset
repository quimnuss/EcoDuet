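; Tutorial game mode for EcoDuet that advances the tutorial as species elders are added.
; On begin play it silences ambient sounds, clears both ecologists' toolbox abilities after a short delay, and relays tutorial step changes to the elder-birth dispatcher.
; AddElder increments and broadcasts the step for Fox, Grass, Pig or Stag.
; Grass also fades ambient sounds in over randomized durations and reveals the water zone mesh.
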(event `self.ReceiveBeginPlay`
  (bind _ecologist_2 (`self.Ecologist 2`))
  (`parent.ReceiveBeginPlay`)
  (`|ExecutionSequence`
    (:`then_0`
      (bind _outactors (`GameplayStatics.GetAllActorsOfClass` "/Script/Engine.AmbientSound"))
      (bind _output_get (set `self.AmbientSounds` _outactors))
      (for _array_element _output_get
        (`AudioComponent.Stop` (`AmbientSound.AudioComponent` _array_element))))
    (:`then_1`
      (add `self.TutorialStepChange` (delegate `ElderBirthDispatch`)))
    (:`then_2`
      (`KismetSystemLibrary.Delay` 0.2)
      (`/Game/EcoDuet/Actors/BP_EcoToolBox.ClearAbilities` (`/Game/EcoDuet/Player/BP_EcoCharacter.ToolBox` (`self.Ecologist 1`)))
      (`/Engine/EditorBlueprintResources/StandardMacros.IsValid` _ecologist_2
        (:`Is Valid`
          (`/Game/EcoDuet/Actors/BP_EcoToolBox.ClearAbilities` (`/Game/EcoDuet/Player/BP_EcoCharacter.ToolBox` _ecologist_2)))))))

(event `ElderBirthDispatch`
  ;[1 1 1] Elder Birth Dispatcher should be at parent
  (`self.ElderBirthDispatcher`))

(fn `AddElder`
  (params (NewElder :type "/Game/EcoDuet/Fauna/BP_EcoElderBaseSpecies Object Reference"))
  (bind _tutorialstep (`self.TutorialStep`))
  (`parent.AddElder` NewElder)
  (switch `EEcoSpeciesType` (`/Game/EcoDuet/Fauna/BP_EcoElderBaseSpecies.EcoSpecies` NewElder)
    (:`EcoFox`
      (`/Engine/EditorBlueprintResources/StandardMacros.IncrementInt` _tutorialstep :!label _label
        (:`  `
          (`self.TutorialStepChange`))))
    (:`EcoGrass`
      (`/Engine/EditorBlueprintResources/StandardMacros.IncrementInt` _tutorialstep
        (:`  `
          (`self.TutorialStepChange`)
          (for _array_element (`self.AmbientSounds`)
            (`AudioComponent.FadeIn` (`AmbientSound.AudioComponent` _array_element) (+ (* (`KismetMathLibrary.RandomFloat`) 30.0) 10.0) 1.0 0.0 "Logarithmic")
            (bind _returnvalue (`GameplayStatics.GetActorOfClass` "/Script/Water.WaterZone"))
            (`SceneComponent.SetVisibility` (`WaterZone.WaterMesh` _returnvalue) true false)))))
    (:`EcoPig`
      (goto _label))
    (:`EcoStag`
      (goto _label))))

(fn `UserConstructionScript`
  (`parent.UserConstructionScript`))