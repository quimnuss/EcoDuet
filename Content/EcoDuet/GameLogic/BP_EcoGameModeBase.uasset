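; Base game mode for EcoDuet that spawns one or two local co-op ecologist characters and manages the pause and help menu.
; It suppresses default pawn spawning, spawning and possessing the character type stored in the game instance, creating a second local player if needed.
; Characters are written back to the game instance, which loads persistent data.
; Menu events toggle pause and input mode; others handle saving and restarting.
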(event `self.ReceiveBeginPlay`
  (bind _asbp_eco_game_instance (cast `/Game/EcoDuet/GameLogic/Bp_EcoGameInstance` (`GameplayStatics.GetGameInstance`) :!pure true))
  (bind _asbp_eco_game_instance_2 (cast `/Game/EcoDuet/GameLogic/Bp_EcoGameInstance` (`GameplayStatics.GetGameInstance`) :!pure true))
  (`/Engine/EditorBlueprintResources/ActorMacros.Switch Has Authority`
    (:`Authority`
      (`|ExecutionSequence`
        (:`then_0`
          ;[1 1 1] Pause menu
          (bind _returnvalue (`|CreateWidget` "/Game/EcoDuet/UI/EcoMenuWidget.EcoMenuWidget_C"))
          (bind _output_get (set `self.Menu` _returnvalue))
          (`Widget.SetVisibility` _output_get "Hidden")
          (`UserWidget.AddToViewport` _output_get 0))
        (:`then_1`
          ;[1 1 1] Store Useful objects
          (set `self.CurrentGameState` (cast `/Game/EcoDuet/GameLogic/BP_EcoGameStateBase` (`GameplayStatics.GetGameState`) :!pure true))
          (bind _outactors (`GameplayStatics.GetAllActorsOfClass` "/Script/Engine.PlayerStart"))
          (set `self.PlayerStarts` _outactors))
        (:`then_2`
          ;[1 1 1] Coop Players start
          (`KismetSystemLibrary.PrintString` "ADD LOCAL PLAYERS")
          (`KismetSystemLibrary.DelayUntilNextTick`)
          (`|ExecutionSequence`
            (:`then_0`
              ;;[1 1 1] we are player 0
              (`/Engine/EditorBlueprintResources/StandardMacros.IsValid` (`self.Ecologist 1`)
                (:`Is Not Valid`
                  (bind _newcharacter (`self.SpawnNewCharacter` 0 (`self.Ecologist 1 Type`)))
                  (bind _output_get_2 (set `/Game/EcoDuet/GameLogic/Bp_EcoGameInstance.Ecologist1` _newcharacter _asbp_eco_game_instance_2))
                  (set `self.Ecologist 1` _output_get_2)
                  (set `/Game/EcoDuet/GameLogic/Bp_EcoGameInstance.EcologistType1` (`self.Ecologist 1 Type`) _asbp_eco_game_instance_2)
                  ;[1 1 1] Persistence
                  (`/Game/EcoDuet/GameLogic/Bp_EcoGameInstance.LoadPersistentData` _asbp_eco_game_instance_2))))
            (:`then_1`
              ;;[1 1 1] we are not player 0
              (`/Engine/EditorBlueprintResources/StandardMacros.IsValid` (`self.Ecologist 2`)
                (:`Is Not Valid`
                  (bind _returnvalue_2 (`self.GetNumPlayers`))
                  (if (> _returnvalue_2 1)
                    (bind _newcharacter_2 (`self.SpawnNewCharacter` 1 (`self.Ecologist 2 Type`) :!label _label))
                    (bind _output_get_3 (set `self.Ecologist 2` _newcharacter_2))
                    (set `/Game/EcoDuet/GameLogic/Bp_EcoGameInstance.Ecologist2` _output_get_3 _asbp_eco_game_instance)
                    (set `/Game/EcoDuet/GameLogic/Bp_EcoGameInstance.EcologistType2` (`self.Ecologist 2 Type`) _asbp_eco_game_instance)
                    (elif (> (`self.EcoRealPlayers`) 1)
                      (`GameplayStatics.CreatePlayer` 1)
                      (goto _label))))))))
        (:`then_3`
          ;[1 1 1] TODO Move this to Home modes
          (`KismetSystemLibrary.DelayUntilNextTick`)
          (bind _returnvalue_3 (`GameplayStatics.GetActorOfClass` "/Game/EcoDuet/Fauna/BP_EcoSpeciesManager.BP_EcoSpeciesManager_C"))
          (set `/Game/EcoDuet/UI/EcoGLVSimpleWidget.GLVManager` _returnvalue_3 (`/Game/EcoDuet/UI/EcoMenuWidget.EcoGLVSimpleWidget` (`self.Menu`))))))))

(event `ShowHelp`
  (bind _returnvalue (`GameplayStatics.GetPlayerController` 0))
  (bind _menu (`self.Menu`))
  ;[1 1 1] Menu
  (`WidgetSwitcher.SetActiveWidgetIndex` (`/Game/EcoDuet/UI/EcoMenuWidget.MainWidgetSwitcher` _menu) 1)
  (`Widget.SetVisibility` _menu "Visible" :!label _label_2)
  (set `PlayerController.bShowMouseCursor` true _returnvalue)
  (`WidgetBlueprintLibrary.SetInputMode_UIOnlyEx` _returnvalue _menu "DoNotLock" true)
  (`GameplayStatics.SetGamePaused` true))

(event `ShowMenu`
  ;[1 1 1] Menu
  (`WidgetSwitcher.SetActiveWidgetIndex` (`/Game/EcoDuet/UI/EcoMenuWidget.MainWidgetSwitcher` (`self.Menu`)) 0)
  (goto _label_2))

(event `HideMenu`
  (bind _returnvalue (`GameplayStatics.GetPlayerController` 0))
  ;[1 1 1] Menu
  (`Widget.SetVisibility` (`self.Menu`) "Hidden" :!label _label_3)
  (set `PlayerController.bShowMouseCursor` false _returnvalue)
  (`WidgetBlueprintLibrary.SetInputMode_GameOnly` _returnvalue true)
  (`GameplayStatics.SetGamePaused` false))

(event `HideHelp`
  ;[1 1 1] Menu
  (goto _label_3))

(event `SaveGame`
  (`|ExecutionSequence`
    (:`then_0`
      (bind _returnvalue (`GameplayStatics.DoesSaveGameExist` "EcoSave"))
      (if (not _returnvalue)
        (`GameplayStatics.CreateSaveGameObject` "/Game/EcoDuet/GameLogic/BP_EcoSaveGame.BP_EcoSaveGame_C")))
    (:`then_1`
      (`/Game/EcoDuet/GameLogic/BP_EcoGameStateBase.UpdateState` (`self.CurrentGameState`)))))

(event `Restart Ecosystem Run`
  (`self.RestartGame` self))

(fn `SpawnDefaultPawnAtTransform`
  (params (NewPlayer :type "Controller Object Reference") (SpawnTransform :type "Transform Structure (by ref)"))
  (returns (ReturnValue :type "Pawn Object Reference"))
  ;[1 1 1] Disable Default Character Spawn
  (return null))

(fn `SpawnNewCharacter`
  (params (LocalPlayerId :type Integer) (EcoCharacterType :type "/Game/EcoDuet/Player/EcoCharacterType Enum" :default "NewEnumerator1"))
  (returns (NewCharacter :type "/Game/EcoDuet/Player/BP_EcoCharacter Object Reference"))
  (locals (PlayerController :type "PlayerController Object Reference") (NewCharacterAux :type "/Game/EcoDuet/Player/BP_EcoCharacter Object Reference"))
  (bind _playercontroller (`local.PlayerController`))
  (bind _returnvalue (`self.GetTransform` (`self.K2_FindPlayerStart` (`local.PlayerController`))))
  (set `local.PlayerController` (`GameplayStatics.GetPlayerControllerFromID` LocalPlayerId))
  (switch `/Game/EcoDuet/Player/EcoCharacterType` EcoCharacterType
    (:`NewEnumerator1`
      (bind _returnvalue_2 (`|SpawnActorFromClass` "/Game/EcoDuet/Player/BP_EcoCharacter.BP_EcoCharacter_C" _returnvalue "AdjustIfPossibleButAlwaysSpawn" "MultiplyWithRoot" null null))
      (set `local.NewCharacterAux` _returnvalue_2)
      (`Controller.Possess` _playercontroller (`local.NewCharacterAux`) :!label _label))
    (:`NewEnumerator0`
      (bind _returnvalue_3 (`|SpawnActorFromClass` "/Game/EcoDuet/Player/BP_EcoKoikoCharacter_Child.BP_EcoKoikoCharacter_Child_C" _returnvalue "AdjustIfPossibleButAlwaysSpawn" "MultiplyWithRoot" null null))
      (set `local.NewCharacterAux` _returnvalue_3)
      (goto _label))
    (:`NewEnumerator2`
      (bind _returnvalue_4 (`|SpawnActorFromClass` (`self.DefaultPawnClass`) _returnvalue "AdjustIfPossibleButAlwaysSpawn" "MultiplyWithRoot" null null))
      (`Controller.Possess` (`local.PlayerController`) _returnvalue_4)))
  (bind _asbp_eco_player_controller (cast `/Game/EcoDuet/Player/BP_EcoPlayerController` _playercontroller))
  (message `EnhancedInputSubsystemInterface.AddMappingContext` (pcsubsystem `EnhancedInputLocalPlayerSubsystem` _asbp_eco_player_controller) "/Game/EcoDuet/Player/Input/EcoPlayerInputContextBase.EcoPlayerInputContextBase" 0 (struct))
  (return (`local.NewCharacterAux`)))

(fn `UserConstructionScript`
  (bind _asbp_eco_game_instance (cast `/Game/EcoDuet/GameLogic/Bp_EcoGameInstance` (`GameplayStatics.GetGameInstance`) :!pure true))
  (set `self.EcoRealPlayers` (`/Game/EcoDuet/GameLogic/Bp_EcoGameInstance.NumEcoPlayers` _asbp_eco_game_instance))
  (set `self.Ecologist 1 Type` (`/Game/EcoDuet/GameLogic/Bp_EcoGameInstance.EcologistType1` _asbp_eco_game_instance))
  (set `self.Ecologist 2 Type` (`/Game/EcoDuet/GameLogic/Bp_EcoGameInstance.EcologistType2` _asbp_eco_game_instance)))