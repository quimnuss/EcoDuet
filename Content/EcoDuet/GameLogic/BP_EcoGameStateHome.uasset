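; BP_EcoGameStateHome is the game state for EcoDuet's home, tracking player poses and environmental health.
; UpdateState rebuilds PlayersPoses from the transforms of every EcoDuetCharacter in the world.
; UpdateHomeStatus adds incoming deltas to Pollution and SoilPH, clamping both to a normalized range.
; Both are events for outside callers; BeginPlay and Tick are unused.
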(event `UpdateState`
  (bind _playersposes (`self.PlayersPoses`))
  (`KismetArrayLibrary.Array_Clear` _playersposes)
  (bind _outactors (`GameplayStatics.GetAllActorsOfClass` "/Script/EcoDuet.EcoDuetCharacter"))
  (for _array_element _outactors
    (`KismetArrayLibrary.Array_Add` _playersposes (`self.GetTransform` _array_element))))

(event `Update Home Status`
  (params (PollutionDelta :type "Float (double-precision)") (SoilPHDelta :type "Float (double-precision)"))
  (set `self.Pollution` (`KismetMathLibrary.FClamp` (+ PollutionDelta (`self.Pollution`))))
  (set `self.SoilPH` (`KismetMathLibrary.FClamp` (+ SoilPHDelta (`self.SoilPH`)))))

(fn `UserConstructionScript`)