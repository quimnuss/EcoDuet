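; Game mode for the EcoDuet tennis dungeon that keeps a Blue versus Red score based on wall ownership.
; On BeginPlay it adds the tennis HUD widget to the viewport and caches every EcoTennisWall in the level.
; Each Tick, UpdateTennisScore recounts the cached walls by their ScoreOwner, and both totals are stored and pushed to the HUD.
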(event `self.ReceiveBeginPlay`
  (`parent.ReceiveBeginPlay`)
  (`|ExecutionSequence`
    (:`then_0`
      (bind _returnvalue (`|CreateWidget` "/Game/EcoDuet/UI/EcoTennisHUDWidget.EcoTennisHUDWidget_C"))
      (bind _output_get (set `self.TennisHUD` _returnvalue))
      (`Widget.SetVisibility` _output_get "Visible")
      (`UserWidget.AddToViewport` _output_get 0))
    (:`then_1`
      (bind _outactors (`GameplayStatics.GetAllActorsOfClass` "/Game/EcoDuet/Actors/EcoTennisWall.EcoTennisWall_C"))
      (set `self.TennisWalls` _outactors))))

(event `self.ReceiveTick`
  (params (DeltaSeconds :type "Float (single-precision)"))
  (bind _tennishud (`self.TennisHUD`))
  (`parent.ReceiveTick` DeltaSeconds)
  (bind (_bluescore _redscore) (`self.UpdateTennisScore`))
  (bind _output_get (set `self.Blue Score` _bluescore))
  (set `/Game/EcoDuet/UI/EcoTennisHUDWidget.BlueScore` _output_get _tennishud)
  (bind _output_get_2 (set `self.Red Score` _redscore))
  (set `/Game/EcoDuet/UI/EcoTennisHUDWidget.RedScore` _output_get_2 _tennishud))

(fn `UpdateTennisScore`
  (returns (BlueScore :type Integer) (RedScore :type Integer))
  (locals (BlueScoreTmp :type Integer) (RedScoreTmp :type Integer))
  (for _array_element (`self.TennisWalls`)
    (switch `int` (`/Game/EcoDuet/Actors/EcoTennisWall.ScoreOwner` _array_element)
      (:`0`
        (`/Engine/EditorBlueprintResources/StandardMacros.IncrementInt` (`local.BlueScoreTmp`)))
      (:`1`
        (`/Engine/EditorBlueprintResources/StandardMacros.IncrementInt` (`local.RedScoreTmp`)))))
  (return (`local.BlueScoreTmp`) (`local.RedScoreTmp`)))

(fn `UserConstructionScript`
  (`parent.UserConstructionScript`))