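; Player character for EcoDuet that interacts with species elders, plants grass and spawns improve-pig cubes.
; An activation sphere picks one target elder and toggles its animal icons, while action events adjust or switch that elder's cubes.
; Planting crouches briefly, spawns a grass child ahead and registers it with the grass elder.
; BeginPlay attaches the audio listener's attenuation to the mesh and displays the player controller ID.
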(event `self.ReceiveBeginPlay`
  (`parent.ReceiveBeginPlay`)
  (bind _asplayer_controller (cast `PlayerController` (`self.GetController`))
    (:`then`
      (`PlayerController.SetAudioListenerAttenuationOverride` _asplayer_controller (`self.Mesh`) (0.0 0.0 0.0))
      (`KismetSystemLibrary.Delay` 0.2)
      (bind _asbp_eco_player_controller (cast `/Game/EcoDuet/Player/BP_EcoPlayerController` (`self.GetController`)))
      (`TextRenderComponent.K2_SetText` (`self.TextRender`) (`KismetTextLibrary.Conv_IntToText` (`GameplayStatics.GetPlayerControllerID` _asbp_eco_player_controller))))
    (:`CastFailed`
      (`KismetSystemLibrary.PrintText` "TODO controller is not a player controller when two players" true true (struct :`G` 0.66 :`B` 1.0 :`A` 1.0) 5.0))))

(event `self.ReceiveTick`
  (params (DeltaSeconds :type "Float (single-precision)"))
  (`parent.ReceiveTick` DeltaSeconds))

(event `Slot1`
  (`self.SpawnInFront` "/Game/EcoDuet/Actors/Bp_EcoImprovePigCube.Bp_EcoImprovePigCube_C" :!label _label))

(event `Slot2`
  (goto _label))

(event `Slot3`
  (goto _label))

(event `ActionPositive`
  (bind _targetelder (`self.TargetElder`))
  (`/Engine/EditorBlueprintResources/StandardMacros.IsValid` _targetelder
    (:`Is Valid`
      (`/Game/EcoDuet/Fauna/BP_EcoElderBaseSpecies.IncreaseCube` _targetelder))))

(event `ActionSwitchAction`
  (bind _targetelder (`self.TargetElder`))
  (`/Engine/EditorBlueprintResources/StandardMacros.IsValid` _targetelder
    (:`Is Valid`
      (`/Game/EcoDuet/Fauna/BP_EcoElderBaseSpecies.ChangeTargetCube` _targetelder true))))

(event `ActionSwitchActionReverse`
  (bind _targetelder (`self.TargetElder`))
  (`/Engine/EditorBlueprintResources/StandardMacros.IsValid` _targetelder
    (:`Is Valid`
      (`/Game/EcoDuet/Fauna/BP_EcoElderBaseSpecies.ChangeTargetCube` _targetelder false))))

(event `ActionNegative`
  (bind _targetelder (`self.TargetElder`))
  (`/Engine/EditorBlueprintResources/StandardMacros.IsValid` _targetelder
    (:`Is Valid`
      (`/Game/EcoDuet/Fauna/BP_EcoElderBaseSpecies.DecreaseCube` _targetelder))))

(event `Plant`
  (bind (_returnvalue_x _returnvalue_y) (`KismetMathLibrary.BreakVector` (`self.K2_GetActorLocation` self)))
  (`self.Crouch` self)
  (`KismetSystemLibrary.Delay` 0.1)
  ;[1 1 1] TODO: put this logic in elder
  (bind _returnvalue (`|SpawnActorFromClass` "/Game/EcoDuet/Fauna/BP_EcoFaunaGrassCharacter_Child.BP_EcoFaunaGrassCharacter_Child_C" (`KismetMathLibrary.Conv_VectorToTransform` (+ (`KismetMathLibrary.MakeVector` _returnvalue_x _returnvalue_y) (* (`self.GetActorForwardVector` self) 100.0))) "AdjustIfPossibleButAlwaysSpawn" "MultiplyWithRoot" null self))
  (bind _returnvalue_2 (`GameplayStatics.GetActorOfClass` "/Game/EcoDuet/Fauna/BP_EcoElderGrassSpecies_Child.BP_EcoElderGrassSpecies_Child_C"))
  (`/Engine/EditorBlueprintResources/StandardMacros.IsValid` _returnvalue_2
    (:`Is Valid`
      (`/Game/EcoDuet/Fauna/BP_EcoElderBaseSpecies.AddEcoFaunaChild` _returnvalue_2 _returnvalue))
    (:`Is Not Valid`
      _))
  (`KismetSystemLibrary.Delay` 0.1)
  (`self.UnCrouch`))

(event `self.ActivationSphereCollision.OnComponentBeginOverlap`
  (params (OverlappedComponent :type "PrimitiveComponent Object Reference") (OtherActor :type "Actor Object Reference") (OtherComp :type "PrimitiveComponent Object Reference") (OtherBodyIndex :type Integer) (bFromSweep :type Boolean) (SweepResult :type "HitResult Structure (by ref)"))
  (`/Engine/EditorBlueprintResources/StandardMacros.IsValid` (`self.TargetElder`)
    (:`Is Not Valid`
      (bind _asbp_eco_elder_base_species (cast `/Game/EcoDuet/Fauna/BP_EcoElderBaseSpecies` OtherActor))
      (bind _output_get (set `self.TargetElder` _asbp_eco_elder_base_species))
      (`/Game/EcoDuet/Fauna/BP_EcoElderBaseSpecies.ShowAnimalIcons` _output_get))))

(event `self.ActivationSphereCollision.OnComponentEndOverlap`
  (params (OverlappedComponent :type "PrimitiveComponent Object Reference") (OtherActor :type "Actor Object Reference") (OtherComp :type "PrimitiveComponent Object Reference") (OtherBodyIndex :type Integer))
  (bind _asbp_eco_elder_base_species (cast `/Game/EcoDuet/Fauna/BP_EcoElderBaseSpecies` OtherActor))
  (if (== (`self.TargetElder`) _asbp_eco_elder_base_species)
    (set `self.TargetElder` null)
    (`/Game/EcoDuet/Fauna/BP_EcoElderBaseSpecies.HideAnimalIcons` _asbp_eco_elder_base_species)))

(fn `SpawnInFront`
  (params (ClassToSpawn :type "Actor Class Reference"))
  (bind _returnvalue (`|SpawnActorFromClass` ClassToSpawn (`KismetMathLibrary.Conv_VectorToTransform` (+ (`self.K2_GetActorLocation` self) (* (`self.GetActorForwardVector` self) 100.0))) "AdjustIfPossibleButAlwaysSpawn" "MultiplyWithRoot" null self))
  (`PrimitiveComponent.AddImpulse` (`self.GetComponentByClass` _returnvalue "/Script/Engine.PrimitiveComponent") (`self.GetActorForwardVector` self) "None" false))

(fn `UserConstructionScript`
  (`parent.UserConstructionScript`))